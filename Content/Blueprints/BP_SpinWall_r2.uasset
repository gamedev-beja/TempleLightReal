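; BP_SpinWall_r2 is a spinning wall that turns its Cylinder by one yaw step each time Activate fires.
; BeginPlay takes the step from the Arrow's relative yaw and sets the DoorOpen timeline's play rate.
; The timeline lerps the rotation, then stores the end angle and resets its time, so turns accumulate.
; An uncalled WakeNearByObjects function sphere-traces around Cube to wake physics bodies, with persistent debug drawing.
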(event EventActivate
  ;[1 1 1] Rotation Code
  (bind _amount (Timeline|DoorOpen Play)
    (:Update
      (Transformation|SetRelativeRotation (Variables|Default|GetCylinder) (Math|Rotator|MakeRotator 0.0 0.0 (Math|Float|Lerp (Variables|Default|GetPrevious%20Rotation) (+ (Variables|Default|GetRotation%20Segment) (Variables|Default|GetPrevious%20Rotation)) _amount)) false false))
    (:Finished
      (Variables|Default|SetPrevious%20Rotation (Math|Float|Lerp (Variables|Default|GetPrevious%20Rotation) (+ (Variables|Default|GetRotation%20Segment) (Variables|Default|GetPrevious%20Rotation)) _amount))
      (Timeline|DoorOpen SetNewTime))))

(event EventBeginPlay
  ;[1 1 1] RotationStart
  (Components|Timeline|SetPlayRate (Variables|Default|GetDoorOpen) (Variables|Default|GetPlayRate))
  (Variables|Default|SetRotation%20Segment (.yaw (Variables|/Script/Engine.SceneComponent|GetRelativeRotation (Variables|Default|GetArrow)))))

(fn ConstructionScript)

(fn WakeNearbyObjects
  (bind _cube (Variables|Default|GetCube))
  (bind _returnvalue (Transformation|GetWorldLocation _cube))
  (bind _outhits (Collision|MultiSphereTraceByChannel _returnvalue _returnvalue 2e+02 "TraceTypeQuery1" false 0 "Persistent"))
  (for _array_element _outhits
    (if (Physics|IsSimulatingPhysics (.HitComponent (Collision|BreakHitResult _array_element)) "None")
      (Class|PrimitiveComponent|WakeAllRigidBodies (.HitComponent (Collision|BreakHitResult _array_element))))))