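; LCD countdown timer prop that shows hours:minutes or minutes:seconds by swapping static meshes on four digits.
; A self-re-entering Gate and Delay loop ticks down once per displayed unit, optionally auto-starting, and sets IsTimerZero at zero.
; Start and Stop events toggle the gate, while Reset restores the initial time.
; The construction script previews that time and applies housing, glass and glow settings through dynamic material instances.
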(event Custom|EventTimerRunOut
  ;[1 1 1] This custom event is triggered when the timer reaches zero
  (Variables|Default|SetIsTimerZero true))

(event Custom|StartTimer
  (bind _customtimecachea (Variables|Default|GetCustomTimeCacheA))
  (bind _customtimecachea_2 (Variables|Default|GetCustomTimeCacheA))
  (bind _returnvalue (/ _customtimecachea 10))
  ;[1 1 1] Call the Start Timer or Stop Timer Events to start/stop the timer during gameplay
  (Utilities|FlowControl|Sequence
    (:then_0
      (goto _label Open))
    (:then_1
      ;[1 1 1] Run the Timer
      (Utilities|FlowControl|Gate (not (Variables|GeneralSettings|GetAutoStartTimer)) :!label _label
        (:Exit
          (Utilities|FlowControl|Delay (Utilities|Select :Index (Variables|GeneralSettings|GetTimerType) :NewEnumerator0 6e+01 :NewEnumerator1 1.0))
          (if (> (Variables|Default|GetCustomTimeCacheB) 0)
            (Math|Integer|DecrementInt (Variables|Default|GetCustomTimeCacheB)
              (:%20%20
                (if (or (!= (Variables|Default|GetCustomTimeCacheB) 0) (!= _customtimecachea_2 0)) :!label _label_2
                  _
                  (else
                    (CallFunction|EventTimerRunOut)))
                (Components|StaticMesh|SetStaticMesh (Variables|Default|GetHourA) (Utilities|Select :Index _returnvalue :Option%200 "/Game/TimersClocksAndCountersPack/Meshes/SM_LCD0.SM_LCD0" :Option%201 "/Game/TimersClocksAndCountersPack/Meshes/SM_LCD1.SM_LCD1" :Option%202 "/Game/TimersClocksAndCountersPack/Meshes/SM_LCD2.SM_LCD2" :Option%203 "/Game/TimersClocksAndCountersPack/Meshes/SM_LCD3.SM_LCD3" :Option%204 "/Game/TimersClocksAndCountersPack/Meshes/SM_LCD4.SM_LCD4" :Option%205 "/Game/TimersClocksAndCountersPack/Meshes/SM_LCD5.SM_LCD5" :Option%206 "/Game/TimersClocksAndCountersPack/Meshes/SM_LCD6.SM_LCD6" :Option%207 "/Game/TimersClocksAndCountersPack/Meshes/SM_LCD7.SM_LCD7" :Option%208 "/Game/TimersClocksAndCountersPack/Meshes/SM_LCD8.SM_LCD8" :Option%209 "/Game/TimersClocksAndCountersPack/Meshes/SM_LCD9.SM_LCD9"))
                (Components|StaticMesh|SetStaticMesh (Variables|Default|GetHourB) (Utilities|Select :Index (- _customtimecachea (* _returnvalue 10)) :Option%200 "/Game/TimersClocksAndCountersPack/Meshes/SM_LCD0.SM_LCD0" :Option%201 "/Game/TimersClocksAndCountersPack/Meshes/SM_LCD1.SM_LCD1" :Option%202 "/Game/TimersClocksAndCountersPack/Meshes/SM_LCD2.SM_LCD2" :Option%203 "/Game/TimersClocksAndCountersPack/Meshes/SM_LCD3.SM_LCD3" :Option%204 "/Game/TimersClocksAndCountersPack/Meshes/SM_LCD4.SM_LCD4" :Option%205 "/Game/TimersClocksAndCountersPack/Meshes/SM_LCD5.SM_LCD5" :Option%206 "/Game/TimersClocksAndCountersPack/Meshes/SM_LCD6.SM_LCD6" :Option%207 "/Game/TimersClocksAndCountersPack/Meshes/SM_LCD7.SM_LCD7" :Option%208 "/Game/TimersClocksAndCountersPack/Meshes/SM_LCD8.SM_LCD8" :Option%209 "/Game/TimersClocksAndCountersPack/Meshes/SM_LCD9.SM_LCD9"))
                (Components|StaticMesh|SetStaticMesh (Variables|Default|GetMinA) (Utilities|Select :Index (/ (Variables|Default|GetCustomTimeCacheB) 10) :Option%200 "/Game/TimersClocksAndCountersPack/Meshes/SM_LCD0.SM_LCD0" :Option%201 "/Game/TimersClocksAndCountersPack/Meshes/SM_LCD1.SM_LCD1" :Option%202 "/Game/TimersClocksAndCountersPack/Meshes/SM_LCD2.SM_LCD2" :Option%203 "/Game/TimersClocksAndCountersPack/Meshes/SM_LCD3.SM_LCD3" :Option%204 "/Game/TimersClocksAndCountersPack/Meshes/SM_LCD4.SM_LCD4" :Option%205 "/Game/TimersClocksAndCountersPack/Meshes/SM_LCD5.SM_LCD5" :Option%206 "/Game/TimersClocksAndCountersPack/Meshes/SM_LCD6.SM_LCD6" :Option%207 "/Game/TimersClocksAndCountersPack/Meshes/SM_LCD7.SM_LCD7" :Option%208 "/Game/TimersClocksAndCountersPack/Meshes/SM_LCD8.SM_LCD8" :Option%209 "/Game/TimersClocksAndCountersPack/Meshes/SM_LCD9.SM_LCD9"))
                (Components|StaticMesh|SetStaticMesh (Variables|Default|GetMinB) (Utilities|Select :Index (- (Variables|Default|GetCustomTimeCacheB) (* (/ (Variables|Default|GetCustomTimeCacheB) 10) 10)) :Option%200 "/Game/TimersClocksAndCountersPack/Meshes/SM_LCD0.SM_LCD0" :Option%201 "/Game/TimersClocksAndCountersPack/Meshes/SM_LCD1.SM_LCD1" :Option%202 "/Game/TimersClocksAndCountersPack/Meshes/SM_LCD2.SM_LCD2" :Option%203 "/Game/TimersClocksAndCountersPack/Meshes/SM_LCD3.SM_LCD3" :Option%204 "/Game/TimersClocksAndCountersPack/Meshes/SM_LCD4.SM_LCD4" :Option%205 "/Game/TimersClocksAndCountersPack/Meshes/SM_LCD5.SM_LCD5" :Option%206 "/Game/TimersClocksAndCountersPack/Meshes/SM_LCD6.SM_LCD6" :Option%207 "/Game/TimersClocksAndCountersPack/Meshes/SM_LCD7.SM_LCD7" :Option%208 "/Game/TimersClocksAndCountersPack/Meshes/SM_LCD8.SM_LCD8" :Option%209 "/Game/TimersClocksAndCountersPack/Meshes/SM_LCD9.SM_LCD9"))
                (goto _label)))
            (elif (> _customtimecachea_2 0)
              (Math|Integer|DecrementInt _customtimecachea_2
                (:%20%20
                  (Variables|Default|SetCustomTimeCacheB 59)
                  (goto _label_2))))))))))

(event Custom|StopTimer
  (bind _customtimecachea (Variables|Default|GetCustomTimeCacheA))
  (bind _customtimecachea_2 (Variables|Default|GetCustomTimeCacheA))
  (bind _returnvalue (/ _customtimecachea 10))
  ;[1 1 1] Call the Start Timer or Stop Timer Events to start/stop the timer during gameplay
  ;[1 1 1] Run the Timer
  (Utilities|FlowControl|Gate (not (Variables|GeneralSettings|GetAutoStartTimer))) ; enters at Close
)

(event Custom|EventUpdateDisplay
  (bind _customtimecachea (Variables|Default|GetCustomTimeCacheA))
  (bind _customtimecacheb (Variables|Default|GetCustomTimeCacheB))
  (bind _returnvalue (/ _customtimecacheb 10))
  (bind _returnvalue_2 (/ _customtimecachea 10))
  ;[1 1 1] Call this Event to update the display of the timer manually
  (Components|StaticMesh|SetStaticMesh (Variables|Default|GetHourA) (Utilities|Select :Index _returnvalue_2 :Option%200 "/Game/TimersClocksAndCountersPack/Meshes/SM_LCD0.SM_LCD0" :Option%201 "/Game/TimersClocksAndCountersPack/Meshes/SM_LCD1.SM_LCD1" :Option%202 "/Game/TimersClocksAndCountersPack/Meshes/SM_LCD2.SM_LCD2" :Option%203 "/Game/TimersClocksAndCountersPack/Meshes/SM_LCD3.SM_LCD3" :Option%204 "/Game/TimersClocksAndCountersPack/Meshes/SM_LCD4.SM_LCD4" :Option%205 "/Game/TimersClocksAndCountersPack/Meshes/SM_LCD5.SM_LCD5" :Option%206 "/Game/TimersClocksAndCountersPack/Meshes/SM_LCD6.SM_LCD6" :Option%207 "/Game/TimersClocksAndCountersPack/Meshes/SM_LCD7.SM_LCD7" :Option%208 "/Game/TimersClocksAndCountersPack/Meshes/SM_LCD8.SM_LCD8" :Option%209 "/Game/TimersClocksAndCountersPack/Meshes/SM_LCD9.SM_LCD9"))
  (Components|StaticMesh|SetStaticMesh (Variables|Default|GetHourB) (Utilities|Select :Index (- _customtimecachea (* _returnvalue_2 10)) :Option%200 "/Game/TimersClocksAndCountersPack/Meshes/SM_LCD0.SM_LCD0" :Option%201 "/Game/TimersClocksAndCountersPack/Meshes/SM_LCD1.SM_LCD1" :Option%202 "/Game/TimersClocksAndCountersPack/Meshes/SM_LCD2.SM_LCD2" :Option%203 "/Game/TimersClocksAndCountersPack/Meshes/SM_LCD3.SM_LCD3" :Option%204 "/Game/TimersClocksAndCountersPack/Meshes/SM_LCD4.SM_LCD4" :Option%205 "/Game/TimersClocksAndCountersPack/Meshes/SM_LCD5.SM_LCD5" :Option%206 "/Game/TimersClocksAndCountersPack/Meshes/SM_LCD6.SM_LCD6" :Option%207 "/Game/TimersClocksAndCountersPack/Meshes/SM_LCD7.SM_LCD7" :Option%208 "/Game/TimersClocksAndCountersPack/Meshes/SM_LCD8.SM_LCD8" :Option%209 "/Game/TimersClocksAndCountersPack/Meshes/SM_LCD9.SM_LCD9"))
  (Components|StaticMesh|SetStaticMesh (Variables|Default|GetMinA) (Utilities|Select :Index _returnvalue :Option%200 "/Game/TimersClocksAndCountersPack/Meshes/SM_LCD0.SM_LCD0" :Option%201 "/Game/TimersClocksAndCountersPack/Meshes/SM_LCD1.SM_LCD1" :Option%202 "/Game/TimersClocksAndCountersPack/Meshes/SM_LCD2.SM_LCD2" :Option%203 "/Game/TimersClocksAndCountersPack/Meshes/SM_LCD3.SM_LCD3" :Option%204 "/Game/TimersClocksAndCountersPack/Meshes/SM_LCD4.SM_LCD4" :Option%205 "/Game/TimersClocksAndCountersPack/Meshes/SM_LCD5.SM_LCD5" :Option%206 "/Game/TimersClocksAndCountersPack/Meshes/SM_LCD6.SM_LCD6" :Option%207 "/Game/TimersClocksAndCountersPack/Meshes/SM_LCD7.SM_LCD7" :Option%208 "/Game/TimersClocksAndCountersPack/Meshes/SM_LCD8.SM_LCD8" :Option%209 "/Game/TimersClocksAndCountersPack/Meshes/SM_LCD9.SM_LCD9"))
  (Components|StaticMesh|SetStaticMesh (Variables|Default|GetMinB) (Utilities|Select :Index (- _customtimecacheb (* _returnvalue 10)) :Option%200 "/Game/TimersClocksAndCountersPack/Meshes/SM_LCD0.SM_LCD0" :Option%201 "/Game/TimersClocksAndCountersPack/Meshes/SM_LCD1.SM_LCD1" :Option%202 "/Game/TimersClocksAndCountersPack/Meshes/SM_LCD2.SM_LCD2" :Option%203 "/Game/TimersClocksAndCountersPack/Meshes/SM_LCD3.SM_LCD3" :Option%204 "/Game/TimersClocksAndCountersPack/Meshes/SM_LCD4.SM_LCD4" :Option%205 "/Game/TimersClocksAndCountersPack/Meshes/SM_LCD5.SM_LCD5" :Option%206 "/Game/TimersClocksAndCountersPack/Meshes/SM_LCD6.SM_LCD6" :Option%207 "/Game/TimersClocksAndCountersPack/Meshes/SM_LCD7.SM_LCD7" :Option%208 "/Game/TimersClocksAndCountersPack/Meshes/SM_LCD8.SM_LCD8" :Option%209 "/Game/TimersClocksAndCountersPack/Meshes/SM_LCD9.SM_LCD9")))

(event Custom|EventResetTimer
  ;[1 1 1] Reset Timer to initial settings
  (Variables|Default|SetCustomTimeCacheA (Utilities|Select :Index (Variables|GeneralSettings|GetTimerType) :NewEnumerator0 (Variables|GeneralSettings|GetInitialTimeHours) :NewEnumerator1 (Variables|GeneralSettings|GetInitialTimeMinutes)))
  (Variables|Default|SetCustomTimeCacheB (Utilities|Select :Index (Variables|GeneralSettings|GetTimerType) :NewEnumerator0 (Variables|GeneralSettings|GetInitialTimeMinutes) :NewEnumerator1 (Variables|GeneralSettings|GetInitialTimeSeconds)))
  (Variables|Default|SetIsTimerZero false)
  (CallFunction|EventUpdateDisplay))

(event EventBeginPlay
  ;[1 1 1] InitialSetup
  (Variables|Default|SetCustomTimeCacheA (Utilities|Select :Index (Variables|GeneralSettings|GetTimerType) :NewEnumerator0 (Variables|GeneralSettings|GetInitialTimeHours) :NewEnumerator1 (Variables|GeneralSettings|GetInitialTimeMinutes)))
  (Variables|Default|SetCustomTimeCacheB (Utilities|Select :Index (Variables|GeneralSettings|GetTimerType) :NewEnumerator0 (Variables|GeneralSettings|GetInitialTimeMinutes) :NewEnumerator1 (Variables|GeneralSettings|GetInitialTimeSeconds)))
  ;[1 1 1] Run the Timer
  (Utilities|FlowControl|Gate (not (Variables|GeneralSettings|GetAutoStartTimer)) :!label _label
    (:Exit
      (Utilities|FlowControl|Delay (Utilities|Select :Index (Variables|GeneralSettings|GetTimerType) :NewEnumerator0 6e+01 :NewEnumerator1 1.0))
      (if (> (Variables|Default|GetCustomTimeCacheB) 0)
        (Math|Integer|DecrementInt (Variables|Default|GetCustomTimeCacheB)
          (:%20%20
            (if (or (!= (Variables|Default|GetCustomTimeCacheB) 0) (!= (Variables|Default|GetCustomTimeCacheA) 0)) :!label _label_2
              _
              (else
                (CallFunction|EventTimerRunOut)))
            (Components|StaticMesh|SetStaticMesh (Variables|Default|GetHourA) (Utilities|Select :Index (/ (Variables|Default|GetCustomTimeCacheA) 10) :Option%200 "/Game/TimersClocksAndCountersPack/Meshes/SM_LCD0.SM_LCD0" :Option%201 "/Game/TimersClocksAndCountersPack/Meshes/SM_LCD1.SM_LCD1" :Option%202 "/Game/TimersClocksAndCountersPack/Meshes/SM_LCD2.SM_LCD2" :Option%203 "/Game/TimersClocksAndCountersPack/Meshes/SM_LCD3.SM_LCD3" :Option%204 "/Game/TimersClocksAndCountersPack/Meshes/SM_LCD4.SM_LCD4" :Option%205 "/Game/TimersClocksAndCountersPack/Meshes/SM_LCD5.SM_LCD5" :Option%206 "/Game/TimersClocksAndCountersPack/Meshes/SM_LCD6.SM_LCD6" :Option%207 "/Game/TimersClocksAndCountersPack/Meshes/SM_LCD7.SM_LCD7" :Option%208 "/Game/TimersClocksAndCountersPack/Meshes/SM_LCD8.SM_LCD8" :Option%209 "/Game/TimersClocksAndCountersPack/Meshes/SM_LCD9.SM_LCD9"))
            (Components|StaticMesh|SetStaticMesh (Variables|Default|GetHourB) (Utilities|Select :Index (- (Variables|Default|GetCustomTimeCacheA) (* (/ (Variables|Default|GetCustomTimeCacheA) 10) 10)) :Option%200 "/Game/TimersClocksAndCountersPack/Meshes/SM_LCD0.SM_LCD0" :Option%201 "/Game/TimersClocksAndCountersPack/Meshes/SM_LCD1.SM_LCD1" :Option%202 "/Game/TimersClocksAndCountersPack/Meshes/SM_LCD2.SM_LCD2" :Option%203 "/Game/TimersClocksAndCountersPack/Meshes/SM_LCD3.SM_LCD3" :Option%204 "/Game/TimersClocksAndCountersPack/Meshes/SM_LCD4.SM_LCD4" :Option%205 "/Game/TimersClocksAndCountersPack/Meshes/SM_LCD5.SM_LCD5" :Option%206 "/Game/TimersClocksAndCountersPack/Meshes/SM_LCD6.SM_LCD6" :Option%207 "/Game/TimersClocksAndCountersPack/Meshes/SM_LCD7.SM_LCD7" :Option%208 "/Game/TimersClocksAndCountersPack/Meshes/SM_LCD8.SM_LCD8" :Option%209 "/Game/TimersClocksAndCountersPack/Meshes/SM_LCD9.SM_LCD9"))
            (Components|StaticMesh|SetStaticMesh (Variables|Default|GetMinA) (Utilities|Select :Index (/ (Variables|Default|GetCustomTimeCacheB) 10) :Option%200 "/Game/TimersClocksAndCountersPack/Meshes/SM_LCD0.SM_LCD0" :Option%201 "/Game/TimersClocksAndCountersPack/Meshes/SM_LCD1.SM_LCD1" :Option%202 "/Game/TimersClocksAndCountersPack/Meshes/SM_LCD2.SM_LCD2" :Option%203 "/Game/TimersClocksAndCountersPack/Meshes/SM_LCD3.SM_LCD3" :Option%204 "/Game/TimersClocksAndCountersPack/Meshes/SM_LCD4.SM_LCD4" :Option%205 "/Game/TimersClocksAndCountersPack/Meshes/SM_LCD5.SM_LCD5" :Option%206 "/Game/TimersClocksAndCountersPack/Meshes/SM_LCD6.SM_LCD6" :Option%207 "/Game/TimersClocksAndCountersPack/Meshes/SM_LCD7.SM_LCD7" :Option%208 "/Game/TimersClocksAndCountersPack/Meshes/SM_LCD8.SM_LCD8" :Option%209 "/Game/TimersClocksAndCountersPack/Meshes/SM_LCD9.SM_LCD9"))
            (Components|StaticMesh|SetStaticMesh (Variables|Default|GetMinB) (Utilities|Select :Index (- (Variables|Default|GetCustomTimeCacheB) (* (/ (Variables|Default|GetCustomTimeCacheB) 10) 10)) :Option%200 "/Game/TimersClocksAndCountersPack/Meshes/SM_LCD0.SM_LCD0" :Option%201 "/Game/TimersClocksAndCountersPack/Meshes/SM_LCD1.SM_LCD1" :Option%202 "/Game/TimersClocksAndCountersPack/Meshes/SM_LCD2.SM_LCD2" :Option%203 "/Game/TimersClocksAndCountersPack/Meshes/SM_LCD3.SM_LCD3" :Option%204 "/Game/TimersClocksAndCountersPack/Meshes/SM_LCD4.SM_LCD4" :Option%205 "/Game/TimersClocksAndCountersPack/Meshes/SM_LCD5.SM_LCD5" :Option%206 "/Game/TimersClocksAndCountersPack/Meshes/SM_LCD6.SM_LCD6" :Option%207 "/Game/TimersClocksAndCountersPack/Meshes/SM_LCD7.SM_LCD7" :Option%208 "/Game/TimersClocksAndCountersPack/Meshes/SM_LCD8.SM_LCD8" :Option%209 "/Game/TimersClocksAndCountersPack/Meshes/SM_LCD9.SM_LCD9"))
            (goto _label)))
        (elif (> (Variables|Default|GetCustomTimeCacheA) 0)
          (Math|Integer|DecrementInt (Variables|Default|GetCustomTimeCacheA)
            (:%20%20
              (Variables|Default|SetCustomTimeCacheB 59)
              (goto _label_2))))))))

(fn ConstructionScript
  (bind _initialtimehours (Variables|GeneralSettings|GetInitialTimeHours))
  (bind _initialtimeminutes (Variables|GeneralSettings|GetInitialTimeMinutes))
  (bind _timertype (Variables|GeneralSettings|GetTimerType))
  (bind _initialtimeminutes_2 (Variables|GeneralSettings|GetInitialTimeMinutes))
  (bind _initialtimeseconds (Variables|GeneralSettings|GetInitialTimeSeconds))
  (bind _housingvariation (Variables|GeneralSettings|GetHousingVariation))
  (bind _housingmesh (Variables|Default|GetHousingMesh))
  (bind _timertype_2 (Variables|GeneralSettings|GetTimerType))
  (bind _returnvalue (!= _housingvariation 0))
  (bind _returnvalue_2 (Utilities|Select :Index _timertype :NewEnumerator0 _initialtimeminutes_2 :NewEnumerator1 _initialtimeseconds))
  (bind _returnvalue_3 (Utilities|Select :Index _timertype_2 :NewEnumerator0 _initialtimehours :NewEnumerator1 _initialtimeminutes))
  (bind _returnvalue_4 (/ _returnvalue_2 10))
  (bind _returnvalue_5 (/ _returnvalue_3 10))
  ;[1 1 1] Apply correct values to all displays
  (Components|StaticMesh|SetStaticMesh (Variables|Default|GetHourA) (Utilities|Select :Index _returnvalue_5 :Option%200 "/Game/TimersClocksAndCountersPack/Meshes/SM_LCD0.SM_LCD0" :Option%201 "/Game/TimersClocksAndCountersPack/Meshes/SM_LCD1.SM_LCD1" :Option%202 "/Game/TimersClocksAndCountersPack/Meshes/SM_LCD2.SM_LCD2" :Option%203 "/Game/TimersClocksAndCountersPack/Meshes/SM_LCD3.SM_LCD3" :Option%204 "/Game/TimersClocksAndCountersPack/Meshes/SM_LCD4.SM_LCD4" :Option%205 "/Game/TimersClocksAndCountersPack/Meshes/SM_LCD5.SM_LCD5" :Option%206 "/Game/TimersClocksAndCountersPack/Meshes/SM_LCD6.SM_LCD6" :Option%207 "/Game/TimersClocksAndCountersPack/Meshes/SM_LCD7.SM_LCD7" :Option%208 "/Game/TimersClocksAndCountersPack/Meshes/SM_LCD8.SM_LCD8" :Option%209 "/Game/TimersClocksAndCountersPack/Meshes/SM_LCD9.SM_LCD9"))
  (Components|StaticMesh|SetStaticMesh (Variables|Default|GetHourB) (Utilities|Select :Index (- _returnvalue_3 (* _returnvalue_5 10)) :Option%200 "/Game/TimersClocksAndCountersPack/Meshes/SM_LCD0.SM_LCD0" :Option%201 "/Game/TimersClocksAndCountersPack/Meshes/SM_LCD1.SM_LCD1" :Option%202 "/Game/TimersClocksAndCountersPack/Meshes/SM_LCD2.SM_LCD2" :Option%203 "/Game/TimersClocksAndCountersPack/Meshes/SM_LCD3.SM_LCD3" :Option%204 "/Game/TimersClocksAndCountersPack/Meshes/SM_LCD4.SM_LCD4" :Option%205 "/Game/TimersClocksAndCountersPack/Meshes/SM_LCD5.SM_LCD5" :Option%206 "/Game/TimersClocksAndCountersPack/Meshes/SM_LCD6.SM_LCD6" :Option%207 "/Game/TimersClocksAndCountersPack/Meshes/SM_LCD7.SM_LCD7" :Option%208 "/Game/TimersClocksAndCountersPack/Meshes/SM_LCD8.SM_LCD8" :Option%209 "/Game/TimersClocksAndCountersPack/Meshes/SM_LCD9.SM_LCD9"))
  (Components|StaticMesh|SetStaticMesh (Variables|Default|GetMinA) (Utilities|Select :Index _returnvalue_4 :Option%200 "/Game/TimersClocksAndCountersPack/Meshes/SM_LCD0.SM_LCD0" :Option%201 "/Game/TimersClocksAndCountersPack/Meshes/SM_LCD1.SM_LCD1" :Option%202 "/Game/TimersClocksAndCountersPack/Meshes/SM_LCD2.SM_LCD2" :Option%203 "/Game/TimersClocksAndCountersPack/Meshes/SM_LCD3.SM_LCD3" :Option%204 "/Game/TimersClocksAndCountersPack/Meshes/SM_LCD4.SM_LCD4" :Option%205 "/Game/TimersClocksAndCountersPack/Meshes/SM_LCD5.SM_LCD5" :Option%206 "/Game/TimersClocksAndCountersPack/Meshes/SM_LCD6.SM_LCD6" :Option%207 "/Game/TimersClocksAndCountersPack/Meshes/SM_LCD7.SM_LCD7" :Option%208 "/Game/TimersClocksAndCountersPack/Meshes/SM_LCD8.SM_LCD8" :Option%209 "/Game/TimersClocksAndCountersPack/Meshes/SM_LCD9.SM_LCD9"))
  (Components|StaticMesh|SetStaticMesh (Variables|Default|GetMinB) (Utilities|Select :Index (- _returnvalue_2 (* _returnvalue_4 10)) :Option%200 "/Game/TimersClocksAndCountersPack/Meshes/SM_LCD0.SM_LCD0" :Option%201 "/Game/TimersClocksAndCountersPack/Meshes/SM_LCD1.SM_LCD1" :Option%202 "/Game/TimersClocksAndCountersPack/Meshes/SM_LCD2.SM_LCD2" :Option%203 "/Game/TimersClocksAndCountersPack/Meshes/SM_LCD3.SM_LCD3" :Option%204 "/Game/TimersClocksAndCountersPack/Meshes/SM_LCD4.SM_LCD4" :Option%205 "/Game/TimersClocksAndCountersPack/Meshes/SM_LCD5.SM_LCD5" :Option%206 "/Game/TimersClocksAndCountersPack/Meshes/SM_LCD6.SM_LCD6" :Option%207 "/Game/TimersClocksAndCountersPack/Meshes/SM_LCD7.SM_LCD7" :Option%208 "/Game/TimersClocksAndCountersPack/Meshes/SM_LCD8.SM_LCD8" :Option%209 "/Game/TimersClocksAndCountersPack/Meshes/SM_LCD9.SM_LCD9"))
  ;[1 1 1] Apply setting as set by the user
  (Rendering|SetVisibility _housingmesh _returnvalue false)
  (Rendering|SetCastShadow _housingmesh _returnvalue)
  (Components|StaticMesh|SetStaticMesh _housingmesh (Utilities|Select :Index _housingvariation :Option%200 "/Game/TimersClocksAndCountersPack/Meshes/SM_LCDHousing01.SM_LCDHousing01" :Option%201 "/Game/TimersClocksAndCountersPack/Meshes/SM_LCDHousing01.SM_LCDHousing01" :Option%202 "/Game/TimersClocksAndCountersPack/Meshes/SM_LCDHousing02.SM_LCDHousing02"))
  (bind _returnvalue_6 (Rendering|Material|CreateDynamicMaterialInstance "/Game/TimersClocksAndCountersPack/Materials/M_LCDNumbers_Inst.M_LCDNumbers_Inst" "None" "None" :!class /Script/Engine.KismetMaterialLibrary))
  (bind _output_get (Variables|Default|SetDynMatLCD _returnvalue_6))
  (Rendering|Material|SetMaterial (Variables|Default|GetSM_LCDColon) 0 _output_get)
  (Rendering|Material|SetScalarParameterValue _output_get "EmissiveMultiplier" (Variables|DisplayAppearance|GetDisplayGlowBrightness) :!class /Script/Engine.MaterialInstanceDynamic)
  (Rendering|Material|SetVectorParameterValue _output_get "GlowColor" (Variables|DisplayAppearance|GetDisplayGlowColor) :!class /Script/Engine.MaterialInstanceDynamic)
  (bind _returnvalue_7 (Rendering|Material|CreateDynamicMaterialInstance "/Game/TimersClocksAndCountersPack/Materials/M_LCDGlass_Inst.M_LCDGlass_Inst" "None" "None" :!class /Script/Engine.KismetMaterialLibrary))
  (bind _output_get_2 (Variables|Default|SetDynMatGlass _returnvalue_7))
  (Rendering|Material|SetMaterial (Variables|Default|GetHousingMesh) 1 _output_get_2)
  (Rendering|Material|SetScalarParameterValue _output_get_2 "OpacityMultiplier" (Variables|GlassAppearance|GetOpacityGlass) :!class /Script/Engine.MaterialInstanceDynamic)
  (Rendering|Material|SetScalarParameterValue _output_get_2 "New-Old" (Variables|GlassAppearance|GetAgeGlass) :!class /Script/Engine.MaterialInstanceDynamic)
  (Rendering|Material|SetScalarParameterValue _output_get_2 "Roughness" (Variables|GlassAppearance|GetRoughnessGlass) :!class /Script/Engine.MaterialInstanceDynamic)
  (Rendering|Material|SetScalarParameterValue _output_get_2 "NormalMapStrength" (Variables|GlassAppearance|GetNormalMapStrengthGlass) :!class /Script/Engine.MaterialInstanceDynamic)
  (bind _returnvalue_8 (Rendering|Material|CreateDynamicMaterialInstance (Utilities|Select :Index (Variables|GeneralSettings|GetHousingMaterial) :NewEnumerator0 "/Game/TimersClocksAndCountersPack/Materials/M_LCDHousing2_Inst.M_LCDHousing2_Inst" :NewEnumerator1 "/Game/TimersClocksAndCountersPack/Materials/M_LCDHousing1_Inst.M_LCDHousing1_Inst") "None" "None" :!class /Script/Engine.KismetMaterialLibrary))
  (bind _output_get_3 (Variables|Default|SetDynMatHousing _returnvalue_8))
  (Rendering|Material|SetMaterial (Variables|Default|GetHousingMesh) 0 _output_get_3)
  (Rendering|Material|SetScalarParameterValue _output_get_3 "New-Old" (Variables|HousingAppearance|GetAgeHousing) :!class /Script/Engine.MaterialInstanceDynamic)
  (Rendering|Material|SetScalarParameterValue _output_get_3 "FadeOutTexture" (Variables|HousingAppearance|GetFadeOutTextureHousing) :!class /Script/Engine.MaterialInstanceDynamic)
  (Rendering|Material|SetScalarParameterValue _output_get_3 "DesaturateTexture" (Variables|HousingAppearance|GetDesaturateTextureHousing) :!class /Script/Engine.MaterialInstanceDynamic)
  (Rendering|Material|SetScalarParameterValue _output_get_3 "Metallic" (Variables|HousingAppearance|GetMetallicHousing) :!class /Script/Engine.MaterialInstanceDynamic)
  (Rendering|Material|SetScalarParameterValue _output_get_3 "Roughness" (Variables|HousingAppearance|GetRoughnessHousing) :!class /Script/Engine.MaterialInstanceDynamic)
  (Rendering|Material|SetScalarParameterValue _output_get_3 "Specular" (Variables|HousingAppearance|GetSpecularHousing) :!class /Script/Engine.MaterialInstanceDynamic)
  (Rendering|Material|SetScalarParameterValue _output_get_3 "NormalMapStrength" (Variables|HousingAppearance|GetNormalMapStrengthHousing) :!class /Script/Engine.MaterialInstanceDynamic)
  (Rendering|Material|SetVectorParameterValue _output_get_3 "Tint" (Variables|HousingAppearance|GetTintHousing) :!class /Script/Engine.MaterialInstanceDynamic))