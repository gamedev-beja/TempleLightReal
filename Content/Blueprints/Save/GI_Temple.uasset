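; GI_Temple is a game instance Blueprint that keeps the player's checkpoint progress in a save game.
; On Init it loads BP_SaveData from the MainSlot slot, or creates a new save object when none exists.
; SaveCheckPoint stores the given checkpoint number in that object and writes it straight back to the slot.
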(event Custom|SaveCheckPoint
  (params (NewCheckPointNum :type Integer))
  (bind _savedata (Variables|Default|GetSaveData))
  (Variables|/Game/Blueprints/Save/BP_SaveData.BP_SaveData_C|SetCheckPointNum _savedata NewCheckPointNum)
  (SaveGame|SaveGametoSlot _savedata "MainSlot"))

(event EventInit
  (bind _returnvalue (SaveGame|DoesSaveGameExist "MainSlot"))
  (if _returnvalue
    (bind _returnvalue_2 (SaveGame|LoadGamefromSlot "MainSlot"))
    (bind _asbp_save_data (Utilities|Casting|CastToBP_SaveData _returnvalue_2))
    (Variables|Default|SetSaveData _asbp_save_data)
    (else
      (bind _returnvalue_3 (SaveGame|CreateSaveGameObject "/Game/Blueprints/Save/BP_SaveData.BP_SaveData_C"))
      (Variables|Default|SetSaveData _returnvalue_3))))