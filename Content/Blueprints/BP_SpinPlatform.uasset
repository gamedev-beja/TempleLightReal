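; BP_SpinPlatform is a platform whose pedestal rotates between zero yaw and a target angle when activated or deactivated.
; The DoorOpen timeline drives a lerp on the pedestal's relative yaw, playing forward on Activate and reversing on Deactivate.
; The Arrow component's relative yaw sets the target angle, and a PlayRate variable sets the timeline speed at BeginPlay.
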(event EventDeactivate
  (bind _amount (Timeline|DoorOpen Reverse)
    (:Update
      (Transformation|SetRelativeRotation (Variables|Default|GetPedestal) (Math|Rotator|MakeRotator 0.0 0.0 (Math|Float|Lerp 0.0 (.yaw (Variables|/Script/Engine.SceneComponent|GetRelativeRotation (Variables|Default|GetArrow))) _amount)) false false))))

(event EventActivate
  (bind _amount (Timeline|DoorOpen Play)
    (:Update
      (Transformation|SetRelativeRotation (Variables|Default|GetPedestal) (Math|Rotator|MakeRotator 0.0 0.0 (Math|Float|Lerp 0.0 (.yaw (Variables|/Script/Engine.SceneComponent|GetRelativeRotation (Variables|Default|GetArrow))) _amount)) false false))))

(event EventBeginPlay
  (Components|Timeline|SetPlayRate (Variables|Default|GetDoorOpen) (Variables|Default|GetPlayRate)))

(fn ConstructionScript)