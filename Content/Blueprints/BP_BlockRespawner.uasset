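; BP_BlockRespawner spawns a reflective block at its own transform when its Activate event fires.
; A boolean chooses between a reflective cube and a reflective angle block.
; An occupied flag blocks further spawns until something ends overlap with the Box component, which clears it without checking which actor left.
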(event OnComponentEndOverlap(Box)
  (params (OverlappedComponent :type Primitive%20Component%20Object%20Reference) (OtherActor :type Actor%20Object%20Reference) (OtherComp :type Primitive%20Component%20Object%20Reference) (OtherBodyIndex :type Integer))
  (Variables|Default|SetIsSpaceOccupied? false))

(event EventActivate
  (if (not (Variables|Default|GetIsSpaceOccupied?))
    (if (not (Variables|Default|GetAngleBlockSpawn?))
      (Game|SpawnActorfromClass "/Game/Blueprints/BP_ReflectiveCube.BP_ReflectiveCube_C" (Transformation|GetActorTransform) "Undefined" 0 0)
      (else
        (Game|SpawnActorfromClass "/Game/Blueprints/BP_ReflectiveAngle.BP_ReflectiveAngle_C" (Transformation|GetActorTransform) "Undefined" 0 0)))
    (Variables|Default|SetIsSpaceOccupied? true)))

(fn ConstructionScript)