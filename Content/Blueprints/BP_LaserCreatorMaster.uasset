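; Laser emitter for reflection puzzles that starts and ends activation on any Bp_GoalSphere its beam hits.
; Each Tick while timed, activated or non-activatable, it line-traces from the Arrow, continuing along hit normals off BPI_Reflective actors up to BounceAmount.
; Mesh actors spawned at BeginPlay are stretched along each segment and hidden when unused.
; Events drive the countdown timer, on/off state and timeline-based stepped yaw rotation.
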(event EventDeactivate
  (Variables|Default|SetActivateTriggered? false))

(event EventActivateTimer
  ;[0.1131 0.8094 1] TimerLoop
  (Variables|Default|SetIsTimerZero? false)
  (Variables|Default|SetCurrentTimerSeconds (Variables|Default|GetTimerAmountSeconds))
  (Utilities|FlowControl|Sequence
    (:then_0
      (goto _label Open))
    (:then_1
      (Utilities|FlowControl|Gate true :!label _label
        (:Exit
          (Utilities|FlowControl|Delay 1.0)
          (bind _result (Math|Float|DecrementFloat (Variables|Default|GetCurrentTimerSeconds))
            (:%20%20
              (Development|PrintString (Utilities|String|ToString(Float) (Variables|Default|GetCurrentTimerSeconds)))
              (if (== _result 0.0)
                (Variables|Default|SetIsTimerZero? true)
                (goto _label Close)
                (else
                  (goto _label))))))))))

(event EventTick
  (params (DeltaSeconds :type Float%20%28single-precision%29))
  (bind _arrow (Variables|Default|GetArrow))
  (if (Math|Boolean|ORBoolean (not (Variables|Default|GetIsTimerZero?)) (Variables|Default|GetActivateTriggered?) (not (Variables|Default|GetActivatable?)))
    ;[0.001214 0.08022 0.4397] Reset these variables every frame
    (Variables|Default|SetLaserOn? true)
    (Variables|Default|SetIsActivating? false)
    (Variables|Default|SetPreviousHit "")
    ;[1 0.272 0.9525] Fire the first laser for the frame
    (CallFunction|BounceLaser (Transformation|GetWorldLocation _arrow) (Math|Vector|GetForwardVector _arrow))
    (CallFunction|CheckifHittingGoal)
    (for _index (range 1 (Variables|Default|GetBounceAmount))
      ;[0.4072 0.1095 0.3864] Continue bouncing lasers up to the BounceAmount
      (if (and (Variables|Default|GetPreviousReturn) (Utilities|DoesObjectImplementInterface (.HitActor (Collision|BreakHitResult (Variables|Default|GetPreviousHit))) "/Game/Blueprints/BPI_Reflective.BPI_Reflective_C"))
        (CallFunction|BounceLaser (.Location (Collision|BreakHitResult (Variables|Default|GetPreviousHit))) (.Normal (Collision|BreakHitResult (Variables|Default|GetPreviousHit))) _index)
        (CallFunction|CheckifHittingGoal)
        (else
          (CallFunction|HideLaserMesh _index))))
    ;[0.02818 0.4985 1] If we are no longer activiting the goal sphere then end the spheres activation and set the variabile to be empty
    (if (not (Variables|Default|GetIsActivating?))
      (Utilities|IsValid (Variables|Default|GetCurrentGoalSphere)
        (:Is%20Valid
          (Default|EndActivation (Variables|Default|GetCurrentGoalSphere))
          (Variables|Default|SetCurrentGoalSphere 0))))
    (else
      ;[1 0.8478 0.05306] If the laser is deactivated then hide all the laser meshes.  Do once is to avoid running this code ccontinuously upon deactivation
      (if (Variables|Default|GetLaserOn?)
        (Utilities|FlowControl|Delay 0.5)
        (Utilities|FlowControl|DoOnce false :!label _label
          (:Completed
            (for _index_2 (range 0 (Variables|Default|GetBounceAmount))
              (CallFunction|HideLaserMesh)
              (Variables|Default|SetLaserOn? false)
              (Utilities|IsValid (Variables|Default|GetCurrentGoalSphere)
                (:Is%20Valid
                  (Default|EndActivation (Variables|Default|GetCurrentGoalSphere))
                  (Variables|Default|SetCurrentGoalSphere 0)
                  (goto _label Reset))
                (:Is%20Not%20Valid
                  (goto _label Reset))))))))))

(event EventActivate
  (Variables|Default|SetActivateTriggered? true))

(event EventBeginPlay
  (Rendering|Material|CreateDynamicMaterialInstance 0 "None" "None" :!class /Script/Engine.KismetMaterialLibrary)
  ;[0.2026 1 0.2461] RotationStart
  (Components|Timeline|SetPlayRate (Variables|Default|GetRotateObject) (Variables|Default|GetPlayRate))
  (Variables|Default|SetRotationSegment (.yaw (Variables|/Script/Engine.SceneComponent|GetRelativeRotation (Variables|Default|GetArrow))))
  ;[1 0.4125 0.252] Create Laser Meshes for Bounces 0-"BounceAmount"
  (for _index (range 0 (Variables|Default|GetBounceAmount))
    (bind _returnvalue (Game|SpawnActorfromClass "/Script/Engine.StaticMeshActor" (Transformation|GetWorldTransform (Variables|Default|GetDefaultSceneRoot)) "Undefined" self 0))
    (Transformation|SetMobility _returnvalue "Movable")
    (Components|StaticMesh|SetStaticMesh (Variables|/Script/Engine.StaticMeshActor|GetStaticMeshComponent _returnvalue) (Variables|Default|GetLaserSMChoice))
    (Utilities|Array|Add (Variables|Default|GetLaserMeshes) _returnvalue)))

(event EventActivateRotation
  ;[0.1832 1 0.2887] Rotation Code
  (if (Variables|Default|GetRotatable?)
    (bind _amount (Timeline|RotateObject Play)
      (:Update
        (Transformation|SetRelativeRotation (Variables|Default|GetSphere) (Math|Rotator|MakeRotator 0.0 0.0 (Math|Float|Lerp (Variables|Default|GetPreviousRotation) (+ (Variables|Default|GetRotationSegment) (Variables|Default|GetPreviousRotation)) _amount)) false false))
      (:Finished
        (Variables|Default|SetPreviousRotation (Math|Float|Lerp (Variables|Default|GetPreviousRotation) (+ (Variables|Default|GetRotationSegment) (Variables|Default|GetPreviousRotation)) _amount))
        (Timeline|RotateObject SetNewTime)))))

(fn ConstructionScript)

(fn AddLaserMesh
  (params (Index :type Integer) (StartLocation :type Vector%20%28by%20ref%29) (EndLocation :type Vector%20%28by%20ref%29))
  (bind _lasermeshes (Variables|Default|GetLaserMeshes))
  (bind _output (Utilities|Array|Get(acopy) _lasermeshes Index))
  (bind _staticmeshcomponent (Variables|/Script/Engine.StaticMeshActor|GetStaticMeshComponent _output))
  (Transformation|SetWorldLocationAndRotation _staticmeshcomponent StartLocation (Math|Rotator|FindLookatRotation StartLocation EndLocation) false false)
  (Transformation|SetRelativeScale3D _staticmeshcomponent (Math|Vector|MakeVector (/ (Math|Vector|Distance(Vector) EndLocation StartLocation) 1e+01) 1.0 1.0))
  (Rendering|SetActorHiddenInGame _output false))

(fn BounceLaser
  (params (StartLocation :type Vector) (Direction :type Vector) (Index :type Integer))
  (bind (_outhit _returnvalue) (Collision|LineTraceByChannel StartLocation (+ StartLocation (* Direction 1.5e+04)) "TraceTypeQuery1" false (Utilities|Array|MakeArray (.HitActor (Collision|BreakHitResult (Variables|Default|GetPreviousHit)))) "None"))
  (Variables|Default|SetPreviousHit _outhit)
  (Variables|Default|SetPreviousReturn _returnvalue)
  (CallFunction|AddLaserMesh Index (.TraceStart (Collision|BreakHitResult _outhit)) (.Location (Collision|BreakHitResult _outhit)))
  (return))

(fn HideLaserMesh
  (params (Index :type Integer))
  (Rendering|SetActorHiddenInGame (Utilities|Array|Get(acopy) (Variables|Default|GetLaserMeshes) Index) true))

(fn CheckifHittingGoal
  (bind _asbp_goal_sphere (Utilities|Casting|CastToBp_GoalSphere (.HitActor (Collision|BreakHitResult (Variables|Default|GetPreviousHit)))))
  (Default|StartActivation _asbp_goal_sphere)
  (Variables|Default|SetPreviousReturn false)
  (Variables|Default|SetCurrentGoalSphere _asbp_goal_sphere)
  (Variables|Default|SetIsActivating? true))

(fn DotheLasers
  (bind _arrow (Variables|Default|GetArrow))
  (if (Variables|Default|GetActivateTriggered?)
    (Variables|Default|SetIsActivating? false)
    (Variables|Default|SetPreviousHit "")
    (CallFunction|BounceLaser (Transformation|GetWorldLocation _arrow) (Math|Vector|GetForwardVector _arrow))
    (CallFunction|CheckifHittingGoal)
    (for _index (range 1 (Variables|Default|GetBounceAmount))
      (if (and (Variables|Default|GetPreviousReturn) (Utilities|DoesObjectImplementInterface (.HitActor (Collision|BreakHitResult (Variables|Default|GetPreviousHit))) "/Game/Blueprints/BPI_Reflective.BPI_Reflective_C"))
        (CallFunction|BounceLaser (.Location (Collision|BreakHitResult (Variables|Default|GetPreviousHit))) (.Normal (Collision|BreakHitResult (Variables|Default|GetPreviousHit))) _index)
        (CallFunction|CheckifHittingGoal)
        (else
          (CallFunction|HideLaserMesh _index))))
    (if (not (Variables|Default|GetIsActivating?))
      (Utilities|IsValid (Variables|Default|GetCurrentGoalSphere)
        (:Is%20Valid
          (Default|EndActivation (Variables|Default|GetCurrentGoalSphere))
          (Variables|Default|SetCurrentGoalSphere 0))))))