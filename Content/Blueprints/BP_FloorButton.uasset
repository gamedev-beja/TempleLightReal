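; BP_FloorButton is a pressure button that activates linked objects when the first-person character or a physics-simulating component rests on it.
; Box overlaps drive a timeline that lowers or raises Cylinder1 along Z.
; Each ActivateObjects entry implementing BPI_Activatable receives activate or deactivate messages.
; Release happens only after an overlap check confirms no character or simulating component remains in the box.
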(event OnComponentBeginOverlap(Box)
  (params (OverlappedComponent :type Primitive%20Component%20Object%20Reference) (OtherActor :type Actor%20Object%20Reference) (OtherComp :type Primitive%20Component%20Object%20Reference) (OtherBodyIndex :type Integer) (bFromSweep :type Boolean) (SweepResult :type Hit%20Result%20Structure%20%28by%20ref%29))
  (if (or (== (Utilities|GetClass OtherActor) "/Game/Blueprints/FirstPersonCharacter.FirstPersonCharacter_C") (Physics|IsSimulatingPhysics OtherComp "None"))
    (CallFunction|DownAnimation)
    (for _array_element (Variables|Default|GetActivateObjects)
      (if (Utilities|DoesObjectImplementInterface _array_element "/Game/Blueprints/BPI_Activatable.BPI_Activatable_C")
        (Class|BPIActivatable|Activate(Message) _array_element)))))

(event OnComponentEndOverlap(Box)
  (params (OverlappedComponent :type Primitive%20Component%20Object%20Reference) (OtherActor :type Actor%20Object%20Reference) (OtherComp :type Primitive%20Component%20Object%20Reference) (OtherBodyIndex :type Integer))
  (if (and (or (== (Utilities|GetClass OtherActor) "/Game/Blueprints/FirstPersonCharacter.FirstPersonCharacter_C") (Physics|IsSimulatingPhysics OtherComp "None")) (CallFunction|AreThereNotAnyObjectsOntopOfButton))
    (CallFunction|UpAnimation)
    (for _array_element (Variables|Default|GetActivateObjects)
      (if (Utilities|DoesObjectImplementInterface _array_element "/Game/Blueprints/BPI_Activatable.BPI_Activatable_C")
        (Class|BPIActivatable|Deactivate(Message) _array_element)))))

(event Custom|UpAnimation
  (bind _zoffset (Timeline|ButtonDown Reverse)
    (:Update
      (Transformation|SetRelativeLocation (Variables|Default|GetCylinder1) (Math|Vector|MakeVector 0.0 0.0 _zoffset) false false))))

(event Custom|DownAnimation
  (bind _zoffset (Timeline|ButtonDown Play)
    (:Update
      (Transformation|SetRelativeLocation (Variables|Default|GetCylinder1) (Math|Vector|MakeVector 0.0 0.0 _zoffset) false false))))

(fn ConstructionScript)

(fn AreThereNotAnyObjectsOntopOfButton
  (for _array_element (Class|PrimitiveComponent|GetOverlappingComponents (Variables|Default|GetBox))
    (if (Physics|IsSimulatingPhysics _array_element "None")
      (LocalVariables|SetIsObjectOnButton true)))
  (return (and (not (LocalVariables|GetIsObjectOnButton)) (== (Utilities|Array|Length (Collision|GetOverlappingActors (Variables|Default|GetBox) "/Game/Blueprints/FirstPersonCharacter.FirstPersonCharacter_C" :!class /Script/Engine.PrimitiveComponent)) 0))))