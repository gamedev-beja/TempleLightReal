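; BP_ActivatorVolume is a trigger volume that switches a set of assigned objects on or off when the first-person character enters it.
; On box overlap by a FirstPersonCharacter, it loops through ActivateObjects and messages each one that implements BPI_Activatable.
; The Deactivate flag picks whether the volume sends the activate or deactivate message, keeping targets decoupled through the interface.
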(event OnComponentBeginOverlap(Box)
  (params (OverlappedComponent :type Primitive%20Component%20Object%20Reference) (OtherActor :type Actor%20Object%20Reference) (OtherComp :type Primitive%20Component%20Object%20Reference) (OtherBodyIndex :type Integer) (bFromSweep :type Boolean) (SweepResult :type Hit%20Result%20Structure%20%28by%20ref%29))
  (Utilities|Casting|CastToFirstPersonCharacter OtherActor)
  (if (not (Variables|Default|GetDeactivate?))
    (for _array_element (Variables|Default|GetActivateObjects)
      (if (Utilities|DoesObjectImplementInterface _array_element "/Game/Blueprints/BPI_Activatable.BPI_Activatable_C")
        (Class|BPIActivatable|Activate(Message) _array_element)))
    (else
      (for _array_element_2 (Variables|Default|GetActivateObjects)
        (if (Utilities|DoesObjectImplementInterface _array_element_2 "/Game/Blueprints/BPI_Activatable.BPI_Activatable_C")
          (Class|BPIActivatable|Deactivate(Message) _array_element_2))))))

(event EventBeginPlay)

(event Collision|EventActorBeginOverlap
  (params (OtherActor :type Actor%20Object%20Reference)))

(event EventTick
  (params (DeltaSeconds :type Float%20%28single-precision%29)))

(fn ConstructionScript)