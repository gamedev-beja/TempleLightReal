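; Laser emitter puzzle actor that, once activated, fires a bouncing beam every tick to power goal spheres.
; Line traces continue along the hit normal off BPI_Reflective actors up to BounceAmount, drawn with pooled meshes stretched per segment.
; Hitting a Bp_GoalSphere stops the chain and starts its activation, ending it when the beam leaves.
; ActivateRotation plays a timeline turning the Sphere in yaw steps derived from the Arrow's initial yaw.
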(event EventActivate
  (Variables|Default|SetActivateTriggered? true))

(event EventTick
  (params (DeltaSeconds :type Float%20%28single-precision%29))
  (bind _arrow (Variables|Default|GetArrow))
  (if (Variables|Default|GetActivateTriggered?)
    (Variables|Default|SetIsActivating? false)
    (Variables|Default|SetPreviousHit "")
    (CallFunction|BounceLaser (Transformation|GetWorldLocation _arrow) (Math|Vector|GetForwardVector _arrow))
    (CallFunction|CheckifHittingGoal)
    (for _index (range 1 (Variables|Default|GetBounceAmount))
      (if (and (Variables|Default|GetPreviousReturn) (Utilities|DoesObjectImplementInterface (.HitActor (Collision|BreakHitResult (Variables|Default|GetPreviousHit))) "/Game/Blueprints/BPI_Reflective.BPI_Reflective_C"))
        (CallFunction|BounceLaser (.Location (Collision|BreakHitResult (Variables|Default|GetPreviousHit))) (.Normal (Collision|BreakHitResult (Variables|Default|GetPreviousHit))) _index)
        (CallFunction|CheckifHittingGoal)
        (else
          (CallFunction|HideLaserMesh _index))))
    (if (not (Variables|Default|GetIsActivating?))
      (Utilities|IsValid (Variables|Default|GetCurrentGoalSphere)
        (:Is%20Valid
          (Default|EndActivation (Variables|Default|GetCurrentGoalSphere))
          (Variables|Default|SetCurrentGoalSphere 0))))))

(event EventBeginPlay
  (for _index (range 0 (Variables|Default|GetBounceAmount))
    (bind _returnvalue (Game|SpawnActorfromClass "/Script/Engine.StaticMeshActor" (Transformation|GetWorldTransform (Variables|Default|GetDefaultSceneRoot)) "Undefined" 0 0))
    (Components|StaticMesh|SetStaticMesh (Variables|/Script/Engine.StaticMeshActor|GetStaticMeshComponent _returnvalue) "/Game/Meshes/SM_LaserMeshActibvate.SM_LaserMeshActibvate")
    (Transformation|SetMobility _returnvalue "Movable")
    (Utilities|Array|Add (Variables|Default|GetLaserMeshes) _returnvalue)
    (Components|Timeline|SetPlayRate (Variables|Default|GetRotateObject) (Variables|Default|GetPlayRate))
    (Variables|Default|SetRotationSegment (.yaw (Variables|/Script/Engine.SceneComponent|GetRelativeRotation (Variables|Default|GetArrow))))))

(event EventActivateRotation
  (bind _rotationsegment (Variables|Default|GetRotationSegment))
  (bind _amount (Timeline|RotateObject Play)
    (:Update
      (Transformation|SetRelativeRotation (Variables|Default|GetSphere) (Math|Rotator|MakeRotator 0.0 0.0 (Math|Float|Lerp (Variables|Default|GetPreviousRotation) (+ _rotationsegment (Variables|Default|GetPreviousRotation)) _amount)) false false)
      (Development|PrintString (Utilities|String|ToString(Float) _rotationsegment)))
    (:Finished
      (Variables|Default|SetPreviousRotation (Math|Float|Lerp (Variables|Default|GetPreviousRotation) (+ _rotationsegment (Variables|Default|GetPreviousRotation)) _amount))
      (Timeline|RotateObject SetNewTime))))

(fn ConstructionScript)

(fn AddLaserMesh
  (params (Index :type Integer) (StartLocation :type Vector%20%28by%20ref%29) (EndLocation :type Vector%20%28by%20ref%29))
  (bind _lasermeshes (Variables|Default|GetLaserMeshes))
  (bind _output (Utilities|Array|Get(acopy) _lasermeshes Index))
  (bind _staticmeshcomponent (Variables|/Script/Engine.StaticMeshActor|GetStaticMeshComponent _output))
  (Transformation|SetWorldLocationAndRotation _staticmeshcomponent StartLocation (Math|Rotator|FindLookatRotation StartLocation EndLocation) false false)
  (Transformation|SetRelativeScale3D _staticmeshcomponent (Math|Vector|MakeVector (/ (Math|Vector|Distance(Vector) EndLocation StartLocation) 1e+01) 1.0 1.0))
  (Rendering|SetActorHiddenInGame _output false))

(fn BounceLaser
  (params (StartLocation :type Vector) (Direction :type Vector) (Index :type Integer))
  (bind (_outhit _returnvalue) (Collision|LineTraceByChannel StartLocation (+ StartLocation (* Direction 1.5e+04)) "TraceTypeQuery1" false (Utilities|Array|MakeArray (.HitActor (Collision|BreakHitResult (Variables|Default|GetPreviousHit)))) "None"))
  (Variables|Default|SetPreviousHit _outhit)
  (Variables|Default|SetPreviousReturn _returnvalue)
  (CallFunction|AddLaserMesh Index (.TraceStart (Collision|BreakHitResult _outhit)) (.Location (Collision|BreakHitResult _outhit)))
  (return))

(fn HideLaserMesh
  (params (Index :type Integer))
  (Rendering|SetActorHiddenInGame (Utilities|Array|Get(acopy) (Variables|Default|GetLaserMeshes) Index) true))

(fn CheckifHittingGoal
  (bind _asbp_goal_sphere (Utilities|Casting|CastToBp_GoalSphere (.HitActor (Collision|BreakHitResult (Variables|Default|GetPreviousHit)))))
  (Default|StartActivation _asbp_goal_sphere)
  (Variables|Default|SetPreviousReturn false)
  (Variables|Default|SetCurrentGoalSphere _asbp_goal_sphere)
  (Variables|Default|SetIsActivating? true))

(fn DotheLasers
  (bind _arrow (Variables|Default|GetArrow))
  (if (Variables|Default|GetActivateTriggered?)
    (Variables|Default|SetIsActivating? false)
    (Variables|Default|SetPreviousHit "")
    (CallFunction|BounceLaser (Transformation|GetWorldLocation _arrow) (Math|Vector|GetForwardVector _arrow))
    (CallFunction|CheckifHittingGoal)
    (for _index (range 1 (Variables|Default|GetBounceAmount))
      (if (and (Variables|Default|GetPreviousReturn) (Utilities|DoesObjectImplementInterface (.HitActor (Collision|BreakHitResult (Variables|Default|GetPreviousHit))) "/Game/Blueprints/BPI_Reflective.BPI_Reflective_C"))
        (CallFunction|BounceLaser (.Location (Collision|BreakHitResult (Variables|Default|GetPreviousHit))) (.Normal (Collision|BreakHitResult (Variables|Default|GetPreviousHit))) _index)
        (CallFunction|CheckifHittingGoal)
        (else
          (CallFunction|HideLaserMesh _index))))
    (if (not (Variables|Default|GetIsActivating?))
      (Utilities|IsValid (Variables|Default|GetCurrentGoalSphere)
        (:Is%20Valid
          (Default|EndActivation (Variables|Default|GetCurrentGoalSphere))
          (Variables|Default|SetCurrentGoalSphere 0))))))