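; Four-digit glowing valve counter prop that counts up or down from an initial number to a target, wrapping between 0 and 9999.
; A gated Delay loop drives the count, with events to start, stop and reset it and to flag target reached.
; Integer division splits the number across four BP_ValveDisplay child actors.
; The construction script previews the initial value and applies mesh variations, dynamic-material settings and glow.
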(event Custom|EventTargetNumberReached
  ;[1 1 1] This Event will be triggered when the target number is reached
  (Variables|Default|SetIsAtTarget true))

(event Custom|EventUpdateDisplay
  (bind _currentnumber (Variables|Default|GetCurrentNumber))
  (bind _returnvalue (/ _currentnumber 1000))
  (bind _returnvalue_2 (/ _currentnumber 100))
  (bind _returnvalue_3 (/ _currentnumber 10))
  (bind _returnvalue_4 (* _returnvalue 100))
  (bind _returnvalue_5 (* _returnvalue 10))
  (bind _returnvalue_6 (- _returnvalue_2 _returnvalue_5))
  (bind _returnvalue_7 (- _returnvalue_3 _returnvalue_4))
  (bind _returnvalue_8 (* _returnvalue_6 10))
  (bind _returnvalue_9 (- _returnvalue_7 _returnvalue_8))
  ;[1 1 1] Updates the display to display the value of "CurrentNumber"
  (bind _asbp_valve_display (Utilities|Casting|CastToBP_ValveDisplay (Variables|/Script/Engine.ChildActorComponent|GetChildActor (Variables|Default|GetThousands))))
  (Variables|/Game/TimersClocksAndCountersPack/Blueprints/BP_ValveDisplay.BP_ValveDisplay_C|SetDisplayNumber _asbp_valve_display _returnvalue)
  (Default|EventApplyValue _asbp_valve_display)
  (bind _asbp_valve_display_2 (Utilities|Casting|CastToBP_ValveDisplay (Variables|/Script/Engine.ChildActorComponent|GetChildActor (Variables|Default|GetHundreds))))
  (Variables|/Game/TimersClocksAndCountersPack/Blueprints/BP_ValveDisplay.BP_ValveDisplay_C|SetDisplayNumber _asbp_valve_display_2 _returnvalue_6)
  (Default|EventApplyValue _asbp_valve_display_2)
  (bind _asbp_valve_display_3 (Utilities|Casting|CastToBP_ValveDisplay (Variables|/Script/Engine.ChildActorComponent|GetChildActor (Variables|Default|GetTens))))
  (Variables|/Game/TimersClocksAndCountersPack/Blueprints/BP_ValveDisplay.BP_ValveDisplay_C|SetDisplayNumber _asbp_valve_display_3 _returnvalue_9)
  (Default|EventApplyValue _asbp_valve_display_3)
  (bind _asbp_valve_display_4 (Utilities|Casting|CastToBP_ValveDisplay (Variables|/Script/Engine.ChildActorComponent|GetChildActor (Variables|Default|GetOnes))))
  (Variables|/Game/TimersClocksAndCountersPack/Blueprints/BP_ValveDisplay.BP_ValveDisplay_C|SetDisplayNumber _asbp_valve_display_4 (- (- (- _currentnumber (* _returnvalue 1000)) (* _returnvalue_6 100)) (* _returnvalue_9 10)))
  (Default|EventApplyValue _asbp_valve_display_4))

(event Custom|StartTimer
  ;[1 1 1] Call the Start Timer or Stop Timer Events to start/stop the timer during gameplay
  (Utilities|FlowControl|Sequence
    (:then_0
      (goto _label Open))
    (:then_1
      ;[1 1 1] Set funtion of counter
      (Utilities|FlowControl|Gate (not (Variables|GeneralSettings|GetAutoStartCounter)) :!label _label
        (:Exit
          (switch Utilities|FlowControl|Switch|SwitchonEnum_CounterFunction (Variables|GeneralSettings|GetCounterFunction)
            (:NewEnumerator1
              (if (!= (Variables|GeneralSettings|GetTargetNumber) (Variables|Default|GetCurrentNumber))
                (Utilities|FlowControl|Delay (Variables|GeneralSettings|GetCounterDelayTime))
                (Math|Integer|IncrementInt (Variables|Default|GetCurrentNumber)
                  (:%20%20
                    (if (> (Variables|Default|GetCurrentNumber) 9999)
                      (Variables|Default|SetCurrentNumber 0))
                    (CallFunction|EventUpdateDisplay :!label _label_2)
                    (goto _label)))
                (else
                  _)))
            (:NewEnumerator2
              (if (!= (Variables|GeneralSettings|GetTargetNumber) (Variables|Default|GetCurrentNumber))
                (Utilities|FlowControl|Delay (Variables|GeneralSettings|GetCounterDelayTime))
                (Math|Integer|DecrementInt (Variables|Default|GetCurrentNumber)
                  (:%20%20
                    (if (< (Variables|Default|GetCurrentNumber) 0)
                      (Variables|Default|SetCurrentNumber 9999)
                      (goto _label_2)
                      (else
                        (goto _label_2)))))
                (else
                  _))))
          (CallFunction|EventTargetNumberReached))))))

(event Custom|StopTimer
  ;[1 1 1] Call the Start Timer or Stop Timer Events to start/stop the timer during gameplay
  ;[1 1 1] Set funtion of counter
  (Utilities|FlowControl|Gate (not (Variables|GeneralSettings|GetAutoStartCounter))) ; enters at Close
)

(event Custom|EventResetCounter
  ;[1 1 1] Call this event to reset the counter to it's initial value.(Call EventStartTimer to start the timer again.)
  (Variables|Default|SetCurrentNumber (Variables|GeneralSettings|GetInitialNumber))
  (Variables|Default|SetIsAtTarget false)
  (CallFunction|EventUpdateDisplay))

(event EventBeginPlay
  ;[1 1 1] Set funtion of counter
  (Variables|Default|SetCurrentNumber (Variables|GeneralSettings|GetInitialNumber))
  (Utilities|FlowControl|Gate (not (Variables|GeneralSettings|GetAutoStartCounter)) :!label _label
    (:Exit
      (switch Utilities|FlowControl|Switch|SwitchonEnum_CounterFunction (Variables|GeneralSettings|GetCounterFunction)
        (:NewEnumerator1
          (if (!= (Variables|GeneralSettings|GetTargetNumber) (Variables|Default|GetCurrentNumber))
            (Utilities|FlowControl|Delay (Variables|GeneralSettings|GetCounterDelayTime))
            (Math|Integer|IncrementInt (Variables|Default|GetCurrentNumber)
              (:%20%20
                (if (> (Variables|Default|GetCurrentNumber) 9999)
                  (Variables|Default|SetCurrentNumber 0))
                (CallFunction|EventUpdateDisplay :!label _label_2)
                (goto _label)))
            (else
              _)))
        (:NewEnumerator2
          (if (!= (Variables|GeneralSettings|GetTargetNumber) (Variables|Default|GetCurrentNumber))
            (Utilities|FlowControl|Delay (Variables|GeneralSettings|GetCounterDelayTime))
            (Math|Integer|DecrementInt (Variables|Default|GetCurrentNumber)
              (:%20%20
                (if (< (Variables|Default|GetCurrentNumber) 0)
                  (Variables|Default|SetCurrentNumber 9999)
                  (goto _label_2)
                  (else
                    (goto _label_2)))))
            (else
              _))))
      (CallFunction|EventTargetNumberReached))))

(fn ConstructionScript
  (bind _addsocket (Variables|GeneralSettings|GetAddSocket))
  (bind _sm_socket04 (Variables|Default|GetSM_Socket04))
  (bind _shieldvariation (Variables|GeneralSettings|GetShieldVariation))
  (bind _sm_shield01 (Variables|Default|GetSM_Shield01))
  (bind _initialnumber (Variables|GeneralSettings|GetInitialNumber))
  (bind _basevariation (Variables|GeneralSettings|GetBaseVariation))
  (bind _sm_valvebase01 (Variables|Default|GetSM_ValveBase01))
  (bind _displayglowbrightness (Variables|Valve,ShieldAndSocketsAppearance|GetDisplayGlowBrightness))
  (bind _displayglowbrightness_2 (Variables|Valve,ShieldAndSocketsAppearance|GetDisplayGlowBrightness))
  (bind _displayglowbrightness_3 (Variables|Valve,ShieldAndSocketsAppearance|GetDisplayGlowBrightness))
  (bind _displayglowbrightness_4 (Variables|Valve,ShieldAndSocketsAppearance|GetDisplayGlowBrightness))
  (bind _returnvalue (!= _shieldvariation 0))
  (bind _returnvalue_2 (!= _basevariation 0))
  (bind _returnvalue_3 (/ _initialnumber 1000))
  (bind _returnvalue_4 (/ _initialnumber 100))
  (bind _returnvalue_5 (/ _initialnumber 10))
  (bind _returnvalue_6 (* _returnvalue_3 100))
  (bind _returnvalue_7 (* _returnvalue_3 10))
  (bind _returnvalue_8 (- _returnvalue_4 _returnvalue_7))
  (bind _returnvalue_9 (- _returnvalue_5 _returnvalue_6))
  (bind _returnvalue_10 (* _returnvalue_8 10))
  (bind _returnvalue_11 (- _returnvalue_9 _returnvalue_10))
  ;[1 1 1] Get System time and apply correct values to all displays
  (bind _asbp_valve_display (Utilities|Casting|CastToBP_ValveDisplay (Variables|/Script/Engine.ChildActorComponent|GetChildActor (Variables|Default|GetThousands))))
  (Variables|/Game/TimersClocksAndCountersPack/Blueprints/BP_ValveDisplay.BP_ValveDisplay_C|SetDisplayNumber _asbp_valve_display _returnvalue_3)
  (Default|EventApplyValue _asbp_valve_display)
  (bind _asbp_valve_display_2 (Utilities|Casting|CastToBP_ValveDisplay (Variables|/Script/Engine.ChildActorComponent|GetChildActor (Variables|Default|GetHundreds))))
  (Variables|/Game/TimersClocksAndCountersPack/Blueprints/BP_ValveDisplay.BP_ValveDisplay_C|SetDisplayNumber _asbp_valve_display_2 _returnvalue_8)
  (Default|EventApplyValue _asbp_valve_display_2)
  (bind _asbp_valve_display_3 (Utilities|Casting|CastToBP_ValveDisplay (Variables|/Script/Engine.ChildActorComponent|GetChildActor (Variables|Default|GetTens))))
  (Variables|/Game/TimersClocksAndCountersPack/Blueprints/BP_ValveDisplay.BP_ValveDisplay_C|SetDisplayNumber _asbp_valve_display_3 _returnvalue_11)
  (Default|EventApplyValue _asbp_valve_display_3)
  (bind _asbp_valve_display_4 (Utilities|Casting|CastToBP_ValveDisplay (Variables|/Script/Engine.ChildActorComponent|GetChildActor (Variables|Default|GetOnes))))
  (Variables|/Game/TimersClocksAndCountersPack/Blueprints/BP_ValveDisplay.BP_ValveDisplay_C|SetDisplayNumber _asbp_valve_display_4 (- (- (- _initialnumber (* _returnvalue_3 1000)) (* _returnvalue_8 100)) (* _returnvalue_11 10)))
  (Default|EventApplyValue _asbp_valve_display_4)
  ;[1 1 1] Apply settings as set by the user
  (Components|StaticMesh|SetStaticMesh _sm_valvebase01 (Utilities|Select :Index _basevariation :Option%200 "/Game/TimersClocksAndCountersPack/Meshes/SM_ValveBase01.SM_ValveBase01" :Option%201 "/Game/TimersClocksAndCountersPack/Meshes/SM_ValveBase01.SM_ValveBase01" :Option%202 "/Game/TimersClocksAndCountersPack/Meshes/SM_ValveBase02.SM_ValveBase02"))
  (Rendering|SetVisibility _sm_valvebase01 _returnvalue_2 false)
  (Rendering|SetCastShadow _sm_valvebase01 _returnvalue_2)
  (Rendering|SetVisibility _sm_socket04 _addsocket false)
  (Rendering|SetCastShadow _sm_socket04 _addsocket)
  (bind _returnvalue_12 (Rendering|Material|CreateDynamicMaterialInstance "/Game/TimersClocksAndCountersPack/Materials/M_Bases01_Inst.M_Bases01_Inst" :!class /Script/Engine.KismetMaterialLibrary))
  (bind _output_get (Variables|Default|SetDynMatBase _returnvalue_12))
  (Rendering|Material|SetMaterial (Variables|Default|GetSM_ValveBase01) 0 _output_get)
  (Rendering|Material|SetScalarParameterValue _output_get "New-Old" (Variables|BaseAppearance|GetAgeBase) :!class /Script/Engine.MaterialInstanceDynamic)
  (Rendering|Material|SetScalarParameterValue _output_get "Metallic" (Variables|BaseAppearance|GetMetallicBase) :!class /Script/Engine.MaterialInstanceDynamic)
  (Rendering|Material|SetScalarParameterValue _output_get "FadeOutTexture" (Variables|BaseAppearance|GetFadeOutTextureBase) :!class /Script/Engine.MaterialInstanceDynamic)
  (Rendering|Material|SetScalarParameterValue _output_get "DesaturateTexture" (Variables|BaseAppearance|GetDesaturateTextureBase) :!class /Script/Engine.MaterialInstanceDynamic)
  (Rendering|Material|SetScalarParameterValue _output_get "Specular" (Variables|BaseAppearance|GetSpecularBase) :!class /Script/Engine.MaterialInstanceDynamic)
  (Rendering|Material|SetScalarParameterValue _output_get "Roughness" (Variables|BaseAppearance|GetRoughnessBase) :!class /Script/Engine.MaterialInstanceDynamic)
  (Rendering|Material|SetVectorParameterValue _output_get "Tint" (Variables|BaseAppearance|GetTintBase) :!class /Script/Engine.MaterialInstanceDynamic)
  (Rendering|Material|SetScalarParameterValue _output_get "NormalMapStrength" (Variables|BaseAppearance|GetNormalMapStrengthBase) :!class /Script/Engine.MaterialInstanceDynamic)
  (bind _returnvalue_13 (Rendering|Material|CreateDynamicMaterialInstance "/Game/TimersClocksAndCountersPack/Materials/M_CounterMetal01_Inst.M_CounterMetal01_Inst" :!class /Script/Engine.KismetMaterialLibrary))
  (bind _output_get_2 (Variables|Default|SetDynMatSocketShield _returnvalue_13))
  (Rendering|Material|SetMaterial (Variables|Default|GetSM_Socket01) 0 _output_get_2)
  (Rendering|Material|SetVectorParameterValue _output_get_2 "Tint" (Variables|Valve,ShieldAndSocketsAppearance|GetTintSocketsAndShield) :!class /Script/Engine.MaterialInstanceDynamic)
  (Rendering|Material|SetScalarParameterValue _output_get_2 "New-Old" (Variables|Valve,ShieldAndSocketsAppearance|GetAgeSocketsAndShield) :!class /Script/Engine.MaterialInstanceDynamic)
  (Rendering|Material|SetScalarParameterValue _output_get_2 "Metallic" (Variables|Valve,ShieldAndSocketsAppearance|GetMetallicSocketsAndShield) :!class /Script/Engine.MaterialInstanceDynamic)
  (Rendering|Material|SetScalarParameterValue _output_get_2 "Roughness" (Variables|Valve,ShieldAndSocketsAppearance|GetRoughnessSocketsAndShield) :!class /Script/Engine.MaterialInstanceDynamic)
  (Rendering|Material|SetScalarParameterValue _output_get_2 "Specular" (Variables|Valve,ShieldAndSocketsAppearance|GetSpecularSocketsAndShield) :!class /Script/Engine.MaterialInstanceDynamic)
  (Rendering|Material|SetScalarParameterValue _output_get_2 "NormalMapStrength" (Variables|Valve,ShieldAndSocketsAppearance|GetNormalMapStrengthSocketsAndShield) :!class /Script/Engine.MaterialInstanceDynamic)
  (Components|StaticMesh|SetStaticMesh _sm_shield01 (Utilities|Select :Index _shieldvariation :Option%200 "/Game/TimersClocksAndCountersPack/Meshes/SM_Shield01.SM_Shield01" :Option%201 "/Game/TimersClocksAndCountersPack/Meshes/SM_Shield01.SM_Shield01" :Option%202 "/Game/TimersClocksAndCountersPack/Meshes/SM_Shield02.SM_Shield02" :Option%203 "/Game/TimersClocksAndCountersPack/Meshes/SM_Shield04.SM_Shield04"))
  (Rendering|SetVisibility _sm_shield01 _returnvalue false)
  (Rendering|SetCastShadow _sm_shield01 _returnvalue)
  (Transformation|SetRelativeScale3D _sm_shield01 (Math|Vector|MakeVector (Utilities|Select :Index _shieldvariation :Option%200 1.0 :Option%201 0.9 :Option%202 0.9 :Option%203 1.0) 1.0 1.0))
  ;[1 1 1] Apply settings to each valve
  (Utilities|FlowControl|Sequence
    (:then_0
      (bind _asbp_valve_display_5 (Utilities|Casting|CastToBP_ValveDisplay (Variables|/Script/Engine.ChildActorComponent|GetChildActor (Variables|Default|GetThousands))))
      (Rendering|Material|SetScalarParameterValue (Variables|/Game/TimersClocksAndCountersPack/Blueprints/BP_ValveDisplay.BP_ValveDisplay_C|GetDynMatValveGlass _asbp_valve_display_5) "New-Old" (Variables|Valve,ShieldAndSocketsAppearance|GetAgeValve) :!class /Script/Engine.MaterialInstanceDynamic)
      (Rendering|Material|SetScalarParameterValue (Variables|/Game/TimersClocksAndCountersPack/Blueprints/BP_ValveDisplay.BP_ValveDisplay_C|GetDynMatValveGlass _asbp_valve_display_5) "Roughness" (Variables|Valve,ShieldAndSocketsAppearance|GetRoughnessValve) :!class /Script/Engine.MaterialInstanceDynamic)
      (Rendering|Material|SetScalarParameterValue (Variables|/Game/TimersClocksAndCountersPack/Blueprints/BP_ValveDisplay.BP_ValveDisplay_C|GetDynMatValveGlass _asbp_valve_display_5) "Specular" (Variables|Valve,ShieldAndSocketsAppearance|GetSpecularValve) :!class /Script/Engine.MaterialInstanceDynamic)
      (Rendering|Material|SetScalarParameterValue (Variables|/Game/TimersClocksAndCountersPack/Blueprints/BP_ValveDisplay.BP_ValveDisplay_C|GetDynMatValveGlass _asbp_valve_display_5) "Metallic" (Variables|Default|GetMetallicValve) :!class /Script/Engine.MaterialInstanceDynamic)
      (Rendering|Material|SetScalarParameterValue (Variables|/Game/TimersClocksAndCountersPack/Blueprints/BP_ValveDisplay.BP_ValveDisplay_C|GetDynMatValveGlass _asbp_valve_display_5) "Normalmapstrength" (Variables|Default|GetNormalMapStrengthValve) :!class /Script/Engine.MaterialInstanceDynamic)
      (Rendering|Material|SetScalarParameterValue (Variables|/Game/TimersClocksAndCountersPack/Blueprints/BP_ValveDisplay.BP_ValveDisplay_C|GetDynMatValveGlass _asbp_valve_display_5) "ReflactiveIndex" (Variables|Valve,ShieldAndSocketsAppearance|GetRefractionValveGlass) :!class /Script/Engine.MaterialInstanceDynamic)
      (Rendering|Material|SetScalarParameterValue (Variables|/Game/TimersClocksAndCountersPack/Blueprints/BP_ValveDisplay.BP_ValveDisplay_C|GetDynMatValveGlass _asbp_valve_display_5) "DesaturateTexture" (Variables|Default|GetValveDesaturateTexture) :!class /Script/Engine.MaterialInstanceDynamic)
      (Rendering|Material|SetVectorParameterValue (Variables|/Game/TimersClocksAndCountersPack/Blueprints/BP_ValveDisplay.BP_ValveDisplay_C|GetDynMatPlate9 _asbp_valve_display_5) "EmissiveColor" (Variables|Valve,ShieldAndSocketsAppearance|GetDisplayGlowColor) :!class /Script/Engine.MaterialInstanceDynamic)
      (if (Variables|/Game/TimersClocksAndCountersPack/Blueprints/BP_ValveDisplay.BP_ValveDisplay_C|GetIsColon _asbp_valve_display_5)
        (Rendering|Material|SetScalarParameterValue (Variables|/Game/TimersClocksAndCountersPack/Blueprints/BP_ValveDisplay.BP_ValveDisplay_C|GetDynMatPlateColon _asbp_valve_display_5) "EmissiveBrightness" (* _displayglowbrightness_2 2.0) :!class /Script/Engine.MaterialInstanceDynamic)
        (else
          (Variables|/Game/TimersClocksAndCountersPack/Blueprints/BP_ValveDisplay.BP_ValveDisplay_C|SetGlowBrightness _asbp_valve_display_5 _displayglowbrightness_2)
          (Rendering|Material|SetScalarParameterValue (Utilities|Select :Index (Variables|/Game/TimersClocksAndCountersPack/Blueprints/BP_ValveDisplay.BP_ValveDisplay_C|GetDisplayNumber _asbp_valve_display_5) :Option%200 (Variables|/Game/TimersClocksAndCountersPack/Blueprints/BP_ValveDisplay.BP_ValveDisplay_C|GetDynMatPlate0 _asbp_valve_display_5) :Option%201 (Variables|/Game/TimersClocksAndCountersPack/Blueprints/BP_ValveDisplay.BP_ValveDisplay_C|GetDynMatPlate1 _asbp_valve_display_5) :Option%202 (Variables|/Game/TimersClocksAndCountersPack/Blueprints/BP_ValveDisplay.BP_ValveDisplay_C|GetDynMatPlate2 _asbp_valve_display_5) :Option%203 (Variables|/Game/TimersClocksAndCountersPack/Blueprints/BP_ValveDisplay.BP_ValveDisplay_C|GetDynMatPlate3 _asbp_valve_display_5) :Option%204 (Variables|/Game/TimersClocksAndCountersPack/Blueprints/BP_ValveDisplay.BP_ValveDisplay_C|GetDynMatPlate4 _asbp_valve_display_5) :Option%205 (Variables|/Game/TimersClocksAndCountersPack/Blueprints/BP_ValveDisplay.BP_ValveDisplay_C|GetDynMatPlate5 _asbp_valve_display_5) :Option%206 (Variables|/Game/TimersClocksAndCountersPack/Blueprints/BP_ValveDisplay.BP_ValveDisplay_C|GetDynMatPlate6 _asbp_valve_display_5) :Option%207 (Variables|/Game/TimersClocksAndCountersPack/Blueprints/BP_ValveDisplay.BP_ValveDisplay_C|GetDynMatPlate7 _asbp_valve_display_5) :Option%208 (Variables|/Game/TimersClocksAndCountersPack/Blueprints/BP_ValveDisplay.BP_ValveDisplay_C|GetDynMatPlate8 _asbp_valve_display_5) :Option%209 (Variables|/Game/TimersClocksAndCountersPack/Blueprints/BP_ValveDisplay.BP_ValveDisplay_C|GetDynMatPlate9 _asbp_valve_display_5)) "EmissiveBrightness" (* (Variables|Valve,ShieldAndSocketsAppearance|GetDisplayGlowBrightness) (Utilities|Select :Index (Variables|/Game/TimersClocksAndCountersPack/Blueprints/BP_ValveDisplay.BP_ValveDisplay_C|GetDisplayNumber _asbp_valve_display_5) :Option%200 11.0 :Option%201 1.0 :Option%202 1.0 :Option%203 1.0 :Option%204 1.3 :Option%205 2.0 :Option%206 3.0 :Option%207 5.0 :Option%208 7.0 :Option%209 8.0)) :!class /Script/Engine.MaterialInstanceDynamic))))
    (:then_1
      (bind _asbp_valve_display_6 (Utilities|Casting|CastToBP_ValveDisplay (Variables|/Script/Engine.ChildActorComponent|GetChildActor (Variables|Default|GetHundreds))))
      (Rendering|Material|SetScalarParameterValue (Variables|/Game/TimersClocksAndCountersPack/Blueprints/BP_ValveDisplay.BP_ValveDisplay_C|GetDynMatValveGlass _asbp_valve_display_6) "New-Old" (Variables|Valve,ShieldAndSocketsAppearance|GetAgeValve) :!class /Script/Engine.MaterialInstanceDynamic)
      (Rendering|Material|SetScalarParameterValue (Variables|/Game/TimersClocksAndCountersPack/Blueprints/BP_ValveDisplay.BP_ValveDisplay_C|GetDynMatValveGlass _asbp_valve_display_6) "Roughness" (Variables|Valve,ShieldAndSocketsAppearance|GetRoughnessValve) :!class /Script/Engine.MaterialInstanceDynamic)
      (Rendering|Material|SetScalarParameterValue (Variables|/Game/TimersClocksAndCountersPack/Blueprints/BP_ValveDisplay.BP_ValveDisplay_C|GetDynMatValveGlass _asbp_valve_display_6) "Specular" (Variables|Valve,ShieldAndSocketsAppearance|GetSpecularValve) :!class /Script/Engine.MaterialInstanceDynamic)
      (Rendering|Material|SetScalarParameterValue (Variables|/Game/TimersClocksAndCountersPack/Blueprints/BP_ValveDisplay.BP_ValveDisplay_C|GetDynMatValveGlass _asbp_valve_display_6) "Metallic" (Variables|Default|GetMetallicValve) :!class /Script/Engine.MaterialInstanceDynamic)
      (Rendering|Material|SetScalarParameterValue (Variables|/Game/TimersClocksAndCountersPack/Blueprints/BP_ValveDisplay.BP_ValveDisplay_C|GetDynMatValveGlass _asbp_valve_display_6) "Normalmapstrength" (Variables|Default|GetNormalMapStrengthValve) :!class /Script/Engine.MaterialInstanceDynamic)
      (Rendering|Material|SetScalarParameterValue (Variables|/Game/TimersClocksAndCountersPack/Blueprints/BP_ValveDisplay.BP_ValveDisplay_C|GetDynMatValveGlass _asbp_valve_display_6) "ReflactiveIndex" (Variables|Valve,ShieldAndSocketsAppearance|GetRefractionValveGlass) :!class /Script/Engine.MaterialInstanceDynamic)
      (Rendering|Material|SetScalarParameterValue (Variables|/Game/TimersClocksAndCountersPack/Blueprints/BP_ValveDisplay.BP_ValveDisplay_C|GetDynMatValveGlass _asbp_valve_display_6) "DesaturateTexture" (Variables|Default|GetValveDesaturateTexture) :!class /Script/Engine.MaterialInstanceDynamic)
      (Rendering|Material|SetVectorParameterValue (Variables|/Game/TimersClocksAndCountersPack/Blueprints/BP_ValveDisplay.BP_ValveDisplay_C|GetDynMatPlate9 _asbp_valve_display_6) "EmissiveColor" (Variables|Valve,ShieldAndSocketsAppearance|GetDisplayGlowColor) :!class /Script/Engine.MaterialInstanceDynamic)
      (if (Variables|/Game/TimersClocksAndCountersPack/Blueprints/BP_ValveDisplay.BP_ValveDisplay_C|GetIsColon _asbp_valve_display_6)
        (Rendering|Material|SetScalarParameterValue (Variables|/Game/TimersClocksAndCountersPack/Blueprints/BP_ValveDisplay.BP_ValveDisplay_C|GetDynMatPlateColon _asbp_valve_display_6) "EmissiveBrightness" (* _displayglowbrightness 2.0) :!class /Script/Engine.MaterialInstanceDynamic)
        (else
          (Variables|/Game/TimersClocksAndCountersPack/Blueprints/BP_ValveDisplay.BP_ValveDisplay_C|SetGlowBrightness _asbp_valve_display_6 _displayglowbrightness)
          (Rendering|Material|SetScalarParameterValue (Utilities|Select :Index (Variables|/Game/TimersClocksAndCountersPack/Blueprints/BP_ValveDisplay.BP_ValveDisplay_C|GetDisplayNumber _asbp_valve_display_6) :Option%200 (Variables|/Game/TimersClocksAndCountersPack/Blueprints/BP_ValveDisplay.BP_ValveDisplay_C|GetDynMatPlate0 _asbp_valve_display_6) :Option%201 (Variables|/Game/TimersClocksAndCountersPack/Blueprints/BP_ValveDisplay.BP_ValveDisplay_C|GetDynMatPlate1 _asbp_valve_display_6) :Option%202 (Variables|/Game/TimersClocksAndCountersPack/Blueprints/BP_ValveDisplay.BP_ValveDisplay_C|GetDynMatPlate2 _asbp_valve_display_6) :Option%203 (Variables|/Game/TimersClocksAndCountersPack/Blueprints/BP_ValveDisplay.BP_ValveDisplay_C|GetDynMatPlate3 _asbp_valve_display_6) :Option%204 (Variables|/Game/TimersClocksAndCountersPack/Blueprints/BP_ValveDisplay.BP_ValveDisplay_C|GetDynMatPlate4 _asbp_valve_display_6) :Option%205 (Variables|/Game/TimersClocksAndCountersPack/Blueprints/BP_ValveDisplay.BP_ValveDisplay_C|GetDynMatPlate5 _asbp_valve_display_6) :Option%206 (Variables|/Game/TimersClocksAndCountersPack/Blueprints/BP_ValveDisplay.BP_ValveDisplay_C|GetDynMatPlate6 _asbp_valve_display_6) :Option%207 (Variables|/Game/TimersClocksAndCountersPack/Blueprints/BP_ValveDisplay.BP_ValveDisplay_C|GetDynMatPlate7 _asbp_valve_display_6) :Option%208 (Variables|/Game/TimersClocksAndCountersPack/Blueprints/BP_ValveDisplay.BP_ValveDisplay_C|GetDynMatPlate8 _asbp_valve_display_6) :Option%209 (Variables|/Game/TimersClocksAndCountersPack/Blueprints/BP_ValveDisplay.BP_ValveDisplay_C|GetDynMatPlate9 _asbp_valve_display_6)) "EmissiveBrightness" (* (Variables|Valve,ShieldAndSocketsAppearance|GetDisplayGlowBrightness) (Utilities|Select :Index (Variables|/Game/TimersClocksAndCountersPack/Blueprints/BP_ValveDisplay.BP_ValveDisplay_C|GetDisplayNumber _asbp_valve_display_6) :Option%200 11.0 :Option%201 1.0 :Option%202 1.0 :Option%203 1.0 :Option%204 1.3 :Option%205 2.0 :Option%206 3.0 :Option%207 5.0 :Option%208 7.0 :Option%209 8.0)) :!class /Script/Engine.MaterialInstanceDynamic))))
    (:then_2
      (bind _asbp_valve_display_7 (Utilities|Casting|CastToBP_ValveDisplay (Variables|/Script/Engine.ChildActorComponent|GetChildActor (Variables|Default|GetTens))))
      (Rendering|Material|SetScalarParameterValue (Variables|/Game/TimersClocksAndCountersPack/Blueprints/BP_ValveDisplay.BP_ValveDisplay_C|GetDynMatValveGlass _asbp_valve_display_7) "New-Old" (Variables|Valve,ShieldAndSocketsAppearance|GetAgeValve) :!class /Script/Engine.MaterialInstanceDynamic)
      (Rendering|Material|SetScalarParameterValue (Variables|/Game/TimersClocksAndCountersPack/Blueprints/BP_ValveDisplay.BP_ValveDisplay_C|GetDynMatValveGlass _asbp_valve_display_7) "Roughness" (Variables|Valve,ShieldAndSocketsAppearance|GetRoughnessValve) :!class /Script/Engine.MaterialInstanceDynamic)
      (Rendering|Material|SetScalarParameterValue (Variables|/Game/TimersClocksAndCountersPack/Blueprints/BP_ValveDisplay.BP_ValveDisplay_C|GetDynMatValveGlass _asbp_valve_display_7) "Specular" (Variables|Valve,ShieldAndSocketsAppearance|GetSpecularValve) :!class /Script/Engine.MaterialInstanceDynamic)
      (Rendering|Material|SetScalarParameterValue (Variables|/Game/TimersClocksAndCountersPack/Blueprints/BP_ValveDisplay.BP_ValveDisplay_C|GetDynMatValveGlass _asbp_valve_display_7) "Metallic" (Variables|Default|GetMetallicValve) :!class /Script/Engine.MaterialInstanceDynamic)
      (Rendering|Material|SetScalarParameterValue (Variables|/Game/TimersClocksAndCountersPack/Blueprints/BP_ValveDisplay.BP_ValveDisplay_C|GetDynMatValveGlass _asbp_valve_display_7) "Normalmapstrength" (Variables|Default|GetNormalMapStrengthValve) :!class /Script/Engine.MaterialInstanceDynamic)
      (Rendering|Material|SetScalarParameterValue (Variables|/Game/TimersClocksAndCountersPack/Blueprints/BP_ValveDisplay.BP_ValveDisplay_C|GetDynMatValveGlass _asbp_valve_display_7) "ReflactiveIndex" (Variables|Valve,ShieldAndSocketsAppearance|GetRefractionValveGlass) :!class /Script/Engine.MaterialInstanceDynamic)
      (Rendering|Material|SetScalarParameterValue (Variables|/Game/TimersClocksAndCountersPack/Blueprints/BP_ValveDisplay.BP_ValveDisplay_C|GetDynMatValveGlass _asbp_valve_display_7) "DesaturateTexture" (Variables|Default|GetValveDesaturateTexture) :!class /Script/Engine.MaterialInstanceDynamic)
      (Rendering|Material|SetVectorParameterValue (Variables|/Game/TimersClocksAndCountersPack/Blueprints/BP_ValveDisplay.BP_ValveDisplay_C|GetDynMatPlate9 _asbp_valve_display_7) "EmissiveColor" (Variables|Valve,ShieldAndSocketsAppearance|GetDisplayGlowColor) :!class /Script/Engine.MaterialInstanceDynamic)
      (if (Variables|/Game/TimersClocksAndCountersPack/Blueprints/BP_ValveDisplay.BP_ValveDisplay_C|GetIsColon _asbp_valve_display_7)
        (Rendering|Material|SetScalarParameterValue (Variables|/Game/TimersClocksAndCountersPack/Blueprints/BP_ValveDisplay.BP_ValveDisplay_C|GetDynMatPlateColon _asbp_valve_display_7) "EmissiveBrightness" (* _displayglowbrightness_3 2.0) :!class /Script/Engine.MaterialInstanceDynamic)
        (else
          (Variables|/Game/TimersClocksAndCountersPack/Blueprints/BP_ValveDisplay.BP_ValveDisplay_C|SetGlowBrightness _asbp_valve_display_7 _displayglowbrightness_3)
          (Rendering|Material|SetScalarParameterValue (Utilities|Select :Index (Variables|/Game/TimersClocksAndCountersPack/Blueprints/BP_ValveDisplay.BP_ValveDisplay_C|GetDisplayNumber _asbp_valve_display_7) :Option%200 (Variables|/Game/TimersClocksAndCountersPack/Blueprints/BP_ValveDisplay.BP_ValveDisplay_C|GetDynMatPlate0 _asbp_valve_display_7) :Option%201 (Variables|/Game/TimersClocksAndCountersPack/Blueprints/BP_ValveDisplay.BP_ValveDisplay_C|GetDynMatPlate1 _asbp_valve_display_7) :Option%202 (Variables|/Game/TimersClocksAndCountersPack/Blueprints/BP_ValveDisplay.BP_ValveDisplay_C|GetDynMatPlate2 _asbp_valve_display_7) :Option%203 (Variables|/Game/TimersClocksAndCountersPack/Blueprints/BP_ValveDisplay.BP_ValveDisplay_C|GetDynMatPlate3 _asbp_valve_display_7) :Option%204 (Variables|/Game/TimersClocksAndCountersPack/Blueprints/BP_ValveDisplay.BP_ValveDisplay_C|GetDynMatPlate4 _asbp_valve_display_7) :Option%205 (Variables|/Game/TimersClocksAndCountersPack/Blueprints/BP_ValveDisplay.BP_ValveDisplay_C|GetDynMatPlate5 _asbp_valve_display_7) :Option%206 (Variables|/Game/TimersClocksAndCountersPack/Blueprints/BP_ValveDisplay.BP_ValveDisplay_C|GetDynMatPlate6 _asbp_valve_display_7) :Option%207 (Variables|/Game/TimersClocksAndCountersPack/Blueprints/BP_ValveDisplay.BP_ValveDisplay_C|GetDynMatPlate7 _asbp_valve_display_7) :Option%208 (Variables|/Game/TimersClocksAndCountersPack/Blueprints/BP_ValveDisplay.BP_ValveDisplay_C|GetDynMatPlate8 _asbp_valve_display_7) :Option%209 (Variables|/Game/TimersClocksAndCountersPack/Blueprints/BP_ValveDisplay.BP_ValveDisplay_C|GetDynMatPlate9 _asbp_valve_display_7)) "EmissiveBrightness" (* (Variables|Valve,ShieldAndSocketsAppearance|GetDisplayGlowBrightness) (Utilities|Select :Index (Variables|/Game/TimersClocksAndCountersPack/Blueprints/BP_ValveDisplay.BP_ValveDisplay_C|GetDisplayNumber _asbp_valve_display_7) :Option%200 11.0 :Option%201 1.0 :Option%202 1.0 :Option%203 1.0 :Option%204 1.3 :Option%205 2.0 :Option%206 3.0 :Option%207 5.0 :Option%208 7.0 :Option%209 8.0)) :!class /Script/Engine.MaterialInstanceDynamic))))
    (:then_3
      (bind _asbp_valve_display_8 (Utilities|Casting|CastToBP_ValveDisplay (Variables|/Script/Engine.ChildActorComponent|GetChildActor (Variables|Default|GetOnes))))
      (Rendering|Material|SetScalarParameterValue (Variables|/Game/TimersClocksAndCountersPack/Blueprints/BP_ValveDisplay.BP_ValveDisplay_C|GetDynMatValveGlass _asbp_valve_display_8) "New-Old" (Variables|Valve,ShieldAndSocketsAppearance|GetAgeValve) :!class /Script/Engine.MaterialInstanceDynamic)
      (Rendering|Material|SetScalarParameterValue (Variables|/Game/TimersClocksAndCountersPack/Blueprints/BP_ValveDisplay.BP_ValveDisplay_C|GetDynMatValveGlass _asbp_valve_display_8) "Roughness" (Variables|Valve,ShieldAndSocketsAppearance|GetRoughnessValve) :!class /Script/Engine.MaterialInstanceDynamic)
      (Rendering|Material|SetScalarParameterValue (Variables|/Game/TimersClocksAndCountersPack/Blueprints/BP_ValveDisplay.BP_ValveDisplay_C|GetDynMatValveGlass _asbp_valve_display_8) "Specular" (Variables|Valve,ShieldAndSocketsAppearance|GetSpecularValve) :!class /Script/Engine.MaterialInstanceDynamic)
      (Rendering|Material|SetScalarParameterValue (Variables|/Game/TimersClocksAndCountersPack/Blueprints/BP_ValveDisplay.BP_ValveDisplay_C|GetDynMatValveGlass _asbp_valve_display_8) "Metallic" (Variables|Default|GetMetallicValve) :!class /Script/Engine.MaterialInstanceDynamic)
      (Rendering|Material|SetScalarParameterValue (Variables|/Game/TimersClocksAndCountersPack/Blueprints/BP_ValveDisplay.BP_ValveDisplay_C|GetDynMatValveGlass _asbp_valve_display_8) "Normalmapstrength" (Variables|Default|GetNormalMapStrengthValve) :!class /Script/Engine.MaterialInstanceDynamic)
      (Rendering|Material|SetScalarParameterValue (Variables|/Game/TimersClocksAndCountersPack/Blueprints/BP_ValveDisplay.BP_ValveDisplay_C|GetDynMatValveGlass _asbp_valve_display_8) "ReflactiveIndex" (Variables|Valve,ShieldAndSocketsAppearance|GetRefractionValveGlass) :!class /Script/Engine.MaterialInstanceDynamic)
      (Rendering|Material|SetScalarParameterValue (Variables|/Game/TimersClocksAndCountersPack/Blueprints/BP_ValveDisplay.BP_ValveDisplay_C|GetDynMatValveGlass _asbp_valve_display_8) "DesaturateTexture" (Variables|Default|GetValveDesaturateTexture) :!class /Script/Engine.MaterialInstanceDynamic)
      (Rendering|Material|SetVectorParameterValue (Variables|/Game/TimersClocksAndCountersPack/Blueprints/BP_ValveDisplay.BP_ValveDisplay_C|GetDynMatPlate9 _asbp_valve_display_8) "EmissiveColor" (Variables|Valve,ShieldAndSocketsAppearance|GetDisplayGlowColor) :!class /Script/Engine.MaterialInstanceDynamic)
      (if (Variables|/Game/TimersClocksAndCountersPack/Blueprints/BP_ValveDisplay.BP_ValveDisplay_C|GetIsColon _asbp_valve_display_8)
        (Rendering|Material|SetScalarParameterValue (Variables|/Game/TimersClocksAndCountersPack/Blueprints/BP_ValveDisplay.BP_ValveDisplay_C|GetDynMatPlateColon _asbp_valve_display_8) "EmissiveBrightness" (* _displayglowbrightness_4 2.0) :!class /Script/Engine.MaterialInstanceDynamic)
        (else
          (Variables|/Game/TimersClocksAndCountersPack/Blueprints/BP_ValveDisplay.BP_ValveDisplay_C|SetGlowBrightness _asbp_valve_display_8 _displayglowbrightness_4)
          (Rendering|Material|SetScalarParameterValue (Utilities|Select :Index (Variables|/Game/TimersClocksAndCountersPack/Blueprints/BP_ValveDisplay.BP_ValveDisplay_C|GetDisplayNumber _asbp_valve_display_8) :Option%200 (Variables|/Game/TimersClocksAndCountersPack/Blueprints/BP_ValveDisplay.BP_ValveDisplay_C|GetDynMatPlate0 _asbp_valve_display_8) :Option%201 (Variables|/Game/TimersClocksAndCountersPack/Blueprints/BP_ValveDisplay.BP_ValveDisplay_C|GetDynMatPlate1 _asbp_valve_display_8) :Option%202 (Variables|/Game/TimersClocksAndCountersPack/Blueprints/BP_ValveDisplay.BP_ValveDisplay_C|GetDynMatPlate2 _asbp_valve_display_8) :Option%203 (Variables|/Game/TimersClocksAndCountersPack/Blueprints/BP_ValveDisplay.BP_ValveDisplay_C|GetDynMatPlate3 _asbp_valve_display_8) :Option%204 (Variables|/Game/TimersClocksAndCountersPack/Blueprints/BP_ValveDisplay.BP_ValveDisplay_C|GetDynMatPlate4 _asbp_valve_display_8) :Option%205 (Variables|/Game/TimersClocksAndCountersPack/Blueprints/BP_ValveDisplay.BP_ValveDisplay_C|GetDynMatPlate5 _asbp_valve_display_8) :Option%206 (Variables|/Game/TimersClocksAndCountersPack/Blueprints/BP_ValveDisplay.BP_ValveDisplay_C|GetDynMatPlate6 _asbp_valve_display_8) :Option%207 (Variables|/Game/TimersClocksAndCountersPack/Blueprints/BP_ValveDisplay.BP_ValveDisplay_C|GetDynMatPlate7 _asbp_valve_display_8) :Option%208 (Variables|/Game/TimersClocksAndCountersPack/Blueprints/BP_ValveDisplay.BP_ValveDisplay_C|GetDynMatPlate8 _asbp_valve_display_8) :Option%209 (Variables|/Game/TimersClocksAndCountersPack/Blueprints/BP_ValveDisplay.BP_ValveDisplay_C|GetDynMatPlate9 _asbp_valve_display_8)) "EmissiveBrightness" (* (Variables|Valve,ShieldAndSocketsAppearance|GetDisplayGlowBrightness) (Utilities|Select :Index (Variables|/Game/TimersClocksAndCountersPack/Blueprints/BP_ValveDisplay.BP_ValveDisplay_C|GetDisplayNumber _asbp_valve_display_8) :Option%200 11.0 :Option%201 1.0 :Option%202 1.0 :Option%203 1.0 :Option%204 1.3 :Option%205 2.0 :Option%206 3.0 :Option%207 5.0 :Option%208 7.0 :Option%209 8.0)) :!class /Script/Engine.MaterialInstanceDynamic))))))